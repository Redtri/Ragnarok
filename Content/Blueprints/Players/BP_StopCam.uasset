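; BP_StopCam is a trigger volume that turns a camera interpolation stop on and off for the X or Y axis, judging by its names.
; Box overlap begin and end send interface calls to set and clear the stop, with X taking priority over Y.
; The X path uses two cross-resetting DoOnce gates to alternate set and clear, while Y is ungated.
; The construction script sizes the box from StopCamBoxExtent.
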(event `self.Box.OnComponentBeginOverlap`
  (params (OverlappedComponent :type "PrimitiveComponent Object Reference") (OtherActor :type "Actor Object Reference") (OtherComp :type "PrimitiveComponent Object Reference") (OtherBodyIndex :type Integer) (bFromSweep :type Boolean) (SweepResult :type "HitResult Structure (by ref)"))
  (bind _stopcaminterpx (`self.StopCamInterpX`))
  (bind _stopcaminterpy (`self.StopCamInterpY`))
  (if _stopcaminterpx
    (`/Engine/EditorBlueprintResources/StandardMacros.DoOnce` false :!label _label
      (:`Completed`
        (`/Game/Blueprints/Players/BPI_StopInterp.InterfaceStopInterpX` _stopcaminterpx)
        (goto _label_2 :!via `Reset`)))
    (elif _stopcaminterpy
      (`/Game/Blueprints/Players/BPI_StopInterp.InterfaceStopInterpY` _stopcaminterpy))))

(event `self.Box.OnComponentEndOverlap`
  (params (OverlappedComponent :type "PrimitiveComponent Object Reference") (OtherActor :type "Actor Object Reference") (OtherComp :type "PrimitiveComponent Object Reference") (OtherBodyIndex :type Integer))
  (if (`self.StopCamInterpX`)
    (`/Engine/EditorBlueprintResources/StandardMacros.DoOnce` false :!label _label_2
      (:`Completed`
        (`/Game/Blueprints/Players/BPI_StopInterp.InterfaceStopInterpX` false)
        (goto _label :!via `Reset`)))
    (elif (`self.StopCamInterpY`)
      (`/Game/Blueprints/Players/BPI_StopInterp.InterfaceStopInterpY` false))))

(fn `UserConstructionScript`
  (`BoxComponent.SetBoxExtent` (`self.Box`) (`self.StopCamBoxExtent`) true))