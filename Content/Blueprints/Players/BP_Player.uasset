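; Player character for a tower defense game, a Paper2D flipbook avatar that moves, attacks rats and builds elemental towers.
; Movement axes orient the interact trigger and switch animations, with building and attacking blocking movement.
; Two element inputs fill a combination shown on the interactable, which Confirm maps to a tower type and spawns on the free spot.
; Random BP_STD sounds play on pooled audio channels, and attack damage lands only when a channel is free.
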(event `Init`
  ;[1 1 1] Init
  (`self.InitializeProperties`))

(event `InputAxis|MoveForward`
  (params (AxisValue :type "Float (single-precision)"))
  (bind _returnvalue (> AxisValue 0.2))
  (bind _interacttrigger (`self.InteractTrigger`))
  (bind _paperflipbook (`self.PaperFlipbook`))
  (bind _m_animations (`self.M Animations`))
  (bind _output_container (break `/Game/Blueprints/Structs/STRUCT_AudioContainer` (`|GetArrayItem` (`self.M Sounds`) (`self.AUD_INDEX_Move`))))
  ;[1 0.1788 0] Moving controls
  (if (and (not (`self.M IsBuilding`)) (not (`self.M IsAttacking`)))
    (if (or (or _returnvalue (< AxisValue -0.2)) (or (< (stale `InputAxis|MoveRight` AxisValue) -0.2) (> (stale `InputAxis|MoveRight` AxisValue) 0.2)))
      (`self.AddMovementInput` (`SceneComponent.GetForwardVector` (`self.Mesh`)) (* (`self.Speed`) AxisValue))
      (if _returnvalue
        ;;[1 1 1] Applies TEUB transform
        (`SceneComponent.K2_SetRelativeLocation` _interacttrigger (515.0 -30.0 0.0) false false)
        (`SceneComponent.K2_SetRelativeRotation` :`self` _interacttrigger :!label _label)
        (if (> AxisValue (`KismetMathLibrary.Abs` (stale `InputAxis|MoveRight` AxisValue))) :!label _label_2
          (`PaperFlipbookComponent.SetFlipbook` _paperflipbook (`|GetArrayItem` _m_animations (`self.INDEX_MoveFront`)))
          (else
            (`PaperFlipbookComponent.SetFlipbook` _paperflipbook (`|GetArrayItem` _m_animations (`self.INDEX_MoveSide`)))))
        (`KismetSystemLibrary.Delay` 0.1)
        (bind _audiosource (`self.GetFreeMovementChannel`))
        (`/Engine/EditorBlueprintResources/StandardMacros.IsValid` _audiosource
          (:`Is Valid`
            (bind _return (`self.GetRandomSoundFrom` _output_container))
            (`AudioComponent.SetSound` _audiosource _return)
            (`AudioComponent.Play` _audiosource 0.0)))
        (elif (< AxisValue -0.2)
          (`SceneComponent.K2_SetRelativeLocation` _interacttrigger (-515.0 -30.0 0.0) false false)
          (goto _label)))
      (else
        (`PaperFlipbookComponent.SetFlipbook` (`self.PaperFlipbook`) (`|GetArrayItem` (`self.M Animations`) (`self.INDEX_IdleFront`)) :!label _label_3)))))

(event `InputAxis|MoveRight`
  (params (AxisValue :type "Float (single-precision)"))
  (bind _returnvalue (> AxisValue 0.2))
  (bind _interacttrigger (`self.InteractTrigger`))
  (bind _paperflipbook (`self.PaperFlipbook`))
  ;[1 0.1788 0] Moving controls
  (if (and (not (`self.M IsBuilding`)) (not (`self.M IsAttacking`)))
    (if (or (or (> (stale `InputAxis|MoveForward` AxisValue) 0.2) (< (stale `InputAxis|MoveForward` AxisValue) -0.2)) (or (< AxisValue -0.2) _returnvalue))
      (`self.AddMovementInput` (`SceneComponent.GetRightVector` (`self.Mesh`)) (* (`self.Speed`) AxisValue))
      (if _returnvalue
        (`SceneComponent.K2_SetRelativeRotation` _paperflipbook (struct :`Yaw` -90.0 :`Roll` 90.0) false false)
        ;;[1 1 1] Applies TEUB transform
        (`SceneComponent.K2_SetRelativeLocation` _interacttrigger (50.0 370.0 0.0) false false)
        (`SceneComponent.K2_SetRelativeRotation` _interacttrigger (struct :`Yaw` 90.0) false false :!label _label_4)
        (goto _label_2)
        (elif (< AxisValue -0.2)
          (`SceneComponent.K2_SetRelativeRotation` _paperflipbook (struct :`Pitch` 180.0 :`Yaw` -90.0 :`Roll` 90.0) false false)
          (`SceneComponent.K2_SetRelativeLocation` _interacttrigger (50.0 -430.0 0.0) false false)
          (goto _label_4)))
      (else
        (goto _label_3)))))

(event `InputAction|Confirm`
  (params (Key :type "Key Structure"))
  (bind (_inputcombination_elem1 _inputcombination_elem2) (break `/Game/Blueprints/Structs/STRUCT_ElemToTowers` (`self.InputCombination`)))
  (bind _m_interactable (`self.M Interactable`))
  (bind _m_towerspot (`/Game/Blueprints/Actors/GameplayElement/BP_InteractionTrigger.M TowerSpot` (`self.M Interactable`)))
  (bind _returnvalue (`self.GetTransform` _m_towerspot))
  (bind _returnvalue_2 (+ (.z (.location _returnvalue)) 500.0))
  ;[1 1 1] Input converted to tower type
  (:`Pressed`
    (if (and (`/Game/Blueprints/Actors/GameplayElement/BP_TowerSpawnPoint.M IsFreeSlot` (`/Game/Blueprints/Actors/GameplayElement/BP_InteractionTrigger.M TowerSpot` _m_interactable)) (`|EnumInequality` _inputcombination_elem1 "NewEnumerator0") (`|EnumInequality` _inputcombination_elem2 "NewEnumerator0"))
      (`/Game/Blueprints/Actors/GameplayElement/BP_InteractionTrigger.Display` _m_interactable false)
      (bind _towertype (`self.InputToTower` (`self.InputCombination`)))
      (switch `/Game/Blueprints/Enums/ENUM_TowerType` _towertype
        (:`NewEnumerator0`
          (bind _returnvalue_3 (`|SpawnActorFromClass` "/Game/Blueprints/Actors/Towers/BP_RangedTower.BP_RangedTower_C" (`KismetMathLibrary.MakeTransform` (`KismetMathLibrary.MakeVector` (.x (.location _returnvalue)) (.y (.location _returnvalue)) _returnvalue_2) (.rotation _returnvalue) (.scale _returnvalue)) "AlwaysSpawn" "OverrideRootScale" null null :!label _label_5))
          (`/Game/Blueprints/Actors/Towers/Parents/BP_BaseTower.Init` _returnvalue_3 _towertype _m_towerspot))
        (:`NewEnumerator1`
          (goto _label_5))
        (:`NewEnumerator2`
          (goto _label_5))
        (:`NewEnumerator3`
          (goto _label_5))
        (:`NewEnumerator4`
          (goto _label_5))
        (:`NewEnumerator5`
          (bind _returnvalue_4 (`|SpawnActorFromClass` "/Game/Blueprints/Actors/Towers/Parents/BP_BaseTower.BP_BaseTower_C" (`KismetMathLibrary.MakeTransform` (`KismetMathLibrary.MakeVector` (.x (.location _returnvalue)) (.y (.location _returnvalue)) _returnvalue_2) (.rotation _returnvalue) (.scale _returnvalue)) "AlwaysSpawn" "OverrideRootScale" null null))
          (`/Game/Blueprints/Actors/Towers/Parents/BP_BaseTower.Init` _returnvalue_4 _towertype _m_towerspot))
        (:`NewEnumerator6`
          (goto _label_5))
        (:`NewEnumerator7`
          (goto _label_5))
        (:`NewEnumerator8`
          (goto _label_5))
        (:`NewEnumerator9`
          (goto _label_5)))
      (set `/Game/Blueprints/Actors/GameplayElement/BP_TowerSpawnPoint.M IsFreeSlot` false _m_towerspot)
      ;;[1 1 1] Building tower
      (`self.BuildTower`)
      (`KismetSystemLibrary.Delay` (- (`PaperFlipbook.GetTotalDuration` (`|GetArrayItem` (`self.M Animations`) (`self.INDEX_Build`))) 0.1))
      (set `self.M IsBuilding` false))))

(event `InputAction|Cancel`
  (params (Key :type "Key Structure"))
  (bind _m_interactable (`self.M Interactable`))
  ;[1 1 1] Input converted to tower type
  (:`Pressed`
    (set `self.InputCombination` (make `/Game/Blueprints/Structs/STRUCT_ElemToTowers` "NewEnumerator0"))
    (`/Game/Blueprints/Actors/GameplayElement/BP_InteractionTrigger.FirstInput` _m_interactable "NewEnumerator0")
    (`/Game/Blueprints/Actors/GameplayElement/BP_InteractionTrigger.SecondInput` _m_interactable "NewEnumerator0")))

(event `self.ReceiveTick`
  (params (DeltaSeconds :type "Float (single-precision)"))
  (bind _returnvalue (`PaperFlipbookComponent.GetFlipbook` (`self.PaperFlipbook`)))
  ;[1 1 1] Scaling up the WONDERFUL GRAPHISTS WORK
  (`SceneComponent.SetWorldScale3D` (`self.PaperFlipbook`) (select `bool` (or (== (`|GetArrayItem` (`self.M Animations`) (`self.INDEX_MoveFront`)) _returnvalue) (== _returnvalue (`|GetArrayItem` (`self.M Animations`) (`self.INDEX_Attack`)))) :`false` (0.15 0.15 0.15) :`true` (0.4 0.4 0.4) :!type "Vector Structure")))

(event `InputAction|Attack`
  (params (Key :type "Key Structure"))
  ;[1 1 1] Attack
  (:`Pressed`
    (if (not (`self.M IsAttacking`))
      (`self.Attack`)
      (`KismetSystemLibrary.Delay` (`PaperFlipbook.GetTotalDuration` (`|GetArrayItem` (`self.M Animations`) (`self.INDEX_Attack`))))
      (set `self.M IsAttacking` false))))

(event `InputAction|Elem_Air`
  (params (Key :type "Key Structure"))
  (bind _m_interactable (`self.M Interactable`))
  (bind _inputcombination_elem1 (break `/Game/Blueprints/Structs/STRUCT_ElemToTowers` (`self.InputCombination`)))
  ;[1 1 1] Input converted to tower type
  ;;[1 1 1] Input combinations
  (:`Pressed`
    (if (`self.M CanInteract`)
      (if (`|EnumEquality` _inputcombination_elem1 "NewEnumerator0")
        (bind _output_get (set `self.InputCombination` (make `/Game/Blueprints/Structs/STRUCT_ElemToTowers` "NewEnumerator2")))
        (`/Game/Blueprints/Actors/GameplayElement/BP_InteractionTrigger.FirstInput` _m_interactable (break `/Game/Blueprints/Structs/STRUCT_ElemToTowers` _output_get))
        (else
          (bind _output_get_2 (set `self.InputCombination` (make `/Game/Blueprints/Structs/STRUCT_ElemToTowers` _inputcombination_elem1 "NewEnumerator2")))
          (`/Game/Blueprints/Actors/GameplayElement/BP_InteractionTrigger.SecondInput` _m_interactable (`.Elem2_6_CA14F8B41F041609001400B79C32386E` (break `/Game/Blueprints/Structs/STRUCT_ElemToTowers` _output_get_2))))))))

(event `InputAction|Elem_Earth`
  (params (Key :type "Key Structure"))
  (bind _m_interactable (`self.M Interactable`))
  (bind _inputcombination_elem1 (break `/Game/Blueprints/Structs/STRUCT_ElemToTowers` (`self.InputCombination`)))
  ;[1 1 1] Input converted to tower type
  ;;[1 1 1] Input combinations
  (:`Pressed`
    (if (`self.M CanInteract`)
      (if (`|EnumEquality` _inputcombination_elem1 "NewEnumerator0")
        (bind _output_get (set `self.InputCombination` (make `/Game/Blueprints/Structs/STRUCT_ElemToTowers` "NewEnumerator3")))
        (`/Game/Blueprints/Actors/GameplayElement/BP_InteractionTrigger.FirstInput` _m_interactable (break `/Game/Blueprints/Structs/STRUCT_ElemToTowers` _output_get))
        (else
          (bind _output_get_2 (set `self.InputCombination` (make `/Game/Blueprints/Structs/STRUCT_ElemToTowers` _inputcombination_elem1 "NewEnumerator3")))
          (`/Game/Blueprints/Actors/GameplayElement/BP_InteractionTrigger.SecondInput` _m_interactable (`.Elem2_6_CA14F8B41F041609001400B79C32386E` (break `/Game/Blueprints/Structs/STRUCT_ElemToTowers` _output_get_2))))))))

(event `InputAction|Elem_Fire`
  (params (Key :type "Key Structure"))
  (bind _m_interactable (`self.M Interactable`))
  (bind _inputcombination_elem1 (break `/Game/Blueprints/Structs/STRUCT_ElemToTowers` (`self.InputCombination`)))
  ;[1 1 1] Input converted to tower type
  ;;[1 1 1] Input combinations
  (:`Pressed`
    (if (`self.M CanInteract`)
      (if (`|EnumEquality` _inputcombination_elem1 "NewEnumerator0")
        (bind _output_get (set `self.InputCombination` (make `/Game/Blueprints/Structs/STRUCT_ElemToTowers` "NewEnumerator1")))
        (`/Game/Blueprints/Actors/GameplayElement/BP_InteractionTrigger.FirstInput` _m_interactable (break `/Game/Blueprints/Structs/STRUCT_ElemToTowers` _output_get))
        (else
          (bind _output_get_2 (set `self.InputCombination` (make `/Game/Blueprints/Structs/STRUCT_ElemToTowers` _inputcombination_elem1 "NewEnumerator1")))
          (`/Game/Blueprints/Actors/GameplayElement/BP_InteractionTrigger.SecondInput` _m_interactable (`.Elem2_6_CA14F8B41F041609001400B79C32386E` (break `/Game/Blueprints/Structs/STRUCT_ElemToTowers` _output_get_2))))))))

(event `InputAction|Elem_Water`
  (params (Key :type "Key Structure"))
  (bind _m_interactable (`self.M Interactable`))
  (bind _inputcombination_elem1 (break `/Game/Blueprints/Structs/STRUCT_ElemToTowers` (`self.InputCombination`)))
  ;[1 1 1] Input converted to tower type
  ;;[1 1 1] Input combinations
  (:`Pressed`
    (if (`self.M CanInteract`)
      (if (`|EnumEquality` _inputcombination_elem1 "NewEnumerator0")
        (bind _output_get (set `self.InputCombination` (make `/Game/Blueprints/Structs/STRUCT_ElemToTowers` "NewEnumerator4")))
        (`/Game/Blueprints/Actors/GameplayElement/BP_InteractionTrigger.FirstInput` _m_interactable (break `/Game/Blueprints/Structs/STRUCT_ElemToTowers` _output_get))
        (else
          (bind _output_get_2 (set `self.InputCombination` (make `/Game/Blueprints/Structs/STRUCT_ElemToTowers` _inputcombination_elem1 "NewEnumerator4")))
          (`/Game/Blueprints/Actors/GameplayElement/BP_InteractionTrigger.SecondInput` _m_interactable (`.Elem2_6_CA14F8B41F041609001400B79C32386E` (break `/Game/Blueprints/Structs/STRUCT_ElemToTowers` _output_get_2))))))))

(fn `Attack`
  (bind _output (`|GetArrayItem` (`self.GetOverlappingActors` "/Game/Blueprints/Actors/Enemy/BP_BaseRat.BP_BaseRat_C")))
  (bind _output_container (break `/Game/Blueprints/Structs/STRUCT_AudioContainer` (`|GetArrayItem` (`self.M Sounds`) (`self.AUD_INDEX_Attack`))))
  (bind _asbp_base_rat (cast `/Game/Blueprints/Actors/Enemy/BP_BaseRat` _output :!pure true))
  (set `self.M IsAttacking` true)
  (`PaperFlipbookComponent.SetFlipbook` (`self.PaperFlipbook`) (`|GetArrayItem` (`self.M Animations`) (`self.INDEX_Attack`)))
  (bind _channel (`self.GetFreeActionChannel`))
  (`/Engine/EditorBlueprintResources/StandardMacros.IsValid` _channel
    (:`Is Valid`
      (bind _return (`self.GetRandomSoundFrom` _output_container))
      (`AudioComponent.SetSound` _channel _return)
      (`AudioComponent.Play` _channel 0.0)
      ;[1 1 1] Damages to the rat
      (`/Engine/EditorBlueprintResources/StandardMacros.IsValid` _output
        (:`Is Valid`
          (bind _stillalive (`/Game/Blueprints/Actors/Enemy/BP_BaseRat.ReceiveDamages` _asbp_base_rat 10.0 0.0 0.0))
          (if _stillalive
            (`/Game/Blueprints/Gamemodes/GM_PlayMode.RemoveRat` (cast `/Game/Blueprints/Gamemodes/GM_PlayMode` (`GameplayStatics.GetGameMode`) :!pure true) _asbp_base_rat true)))))))

(fn `BuildTower`
  (set `self.M IsBuilding` true)
  (`PaperFlipbookComponent.SetFlipbook` (`self.PaperFlipbook`) (`|GetArrayItem` (`self.M Animations`) (`self.INDEX_Build`))))

(fn `GetFreeActionChannel`
  (returns (Channel :type "AudioComponent Object Reference"))
  (bind _channel_action_02 (`self.Channel_Action_02`))
  (bind _channel_action (`self.Channel_Action`))
  (bind _channel_action_01 (`self.Channel_Action_01`))
  (if (`AudioComponent.IsPlaying` _channel_action)
    (if (`AudioComponent.IsPlaying` _channel_action_01)
      (if (`AudioComponent.IsPlaying` _channel_action_02)
        (return null)
        (else
          (return _channel_action_02)))
      (else
        (return _channel_action_01)))
    (else
      (return _channel_action))))

(fn `GetFreeMovementChannel`
  (returns (AudioSource :type "AudioComponent Object Reference"))
  (bind _channel_movement (`self.Channel_Movement`))
  (bind _channel_movement_01 (`self.Channel_Movement_01`))
  (bind _channel_movement_02 (`self.Channel_Movement_02`))
  (if (`AudioComponent.IsPlaying` _channel_movement)
    (if (`AudioComponent.IsPlaying` _channel_movement_01)
      (if (`AudioComponent.IsPlaying` _channel_movement_02)
        (return null)
        (else
          (return _channel_movement_02)))
      (else
        (return _channel_movement_01)))
    (else
      (return _channel_movement))))

(fn `GetRandomSoundFrom`
  (params (Sounds :type "Array of SoundWave Object Reference"))
  (returns (Return :type "SoundWave Object Reference"))
  (return (`|GetArrayItem` Sounds (`KismetMathLibrary.RandomIntegerInRange` 0 (- (`KismetArrayLibrary.Array_Length` Sounds) 1)))))

(fn `InitializeProperties`
  (locals (SoundArray :type "Array of SoundWave Object Reference"))
  (bind _m_animations (`self.M Animations`))
  ;[1 1 1] STD reference
  (bind _outactors (`GameplayStatics.GetAllActorsOfClass` "/Game/Blueprints/Abstract/BP_STD.BP_STD_C"))
  (set `self.M STDRef` (`|GetArrayItem` _outactors))
  ;[1 1 1] Animations
  (`KismetArrayLibrary.Array_Add` _m_animations "/Game/Sprites/Flipbooks/Player/Player_FrontIdle.Player_FrontIdle")
  (`KismetArrayLibrary.Array_Add` _m_animations "/Game/Sprites/Flipbooks/Player/Player_SideIdle.Player_SideIdle")
  (`KismetArrayLibrary.Array_Add` _m_animations "/Game/Sprites/Flipbooks/Player/Player_BackWalk.Player_BackWalk")
  (`KismetArrayLibrary.Array_Add` _m_animations "/Game/Sprites/Flipbooks/Player/Player_SideWalk.Player_SideWalk")
  (`KismetArrayLibrary.Array_Add` _m_animations "/Game/Sprites/Flipbooks/Player/Player_SideAttack.Player_SideAttack")
  (`KismetArrayLibrary.Array_Add` _m_animations "/Game/Sprites/Flipbooks/Player/Player_Building.Player_Building")
  ;[1 1 1] Sounds
  (bind _output_get (set `local.SoundArray` (`/Game/Blueprints/Abstract/BP_STD.M PlayerMoveSounds` (`self.M STDRef`))))
  (`KismetArrayLibrary.Array_Add` (`self.M Sounds`) (make `/Game/Blueprints/Structs/STRUCT_AudioContainer` _output_get))
  (`KismetArrayLibrary.Array_Clear` _output_get)
  (bind _output_get_2 (set `local.SoundArray` (`/Game/Blueprints/Abstract/BP_STD.M PlayerAttackSounds` (`self.M STDRef`))))
  (`KismetArrayLibrary.Array_Add` (`self.M Sounds`) (make `/Game/Blueprints/Structs/STRUCT_AudioContainer` _output_get_2))
  (`KismetArrayLibrary.Array_Clear` _output_get_2))

(fn `InputToTower`
  (params (InputCombination :type "/Game/Blueprints/Structs/STRUCT_ElemToTowers Structure"))
  (returns (TowerType :type "/Game/Blueprints/Enums/ENUM_TowerType Enum"))
  (switch `/Game/Blueprints/Enums/ENUM_Elem` InputCombination_Elem1_4_C9F7FD3328041609000E00D28746D39E
    (:`NewEnumerator1`
      (switch `/Game/Blueprints/Enums/ENUM_Elem` InputCombination_Elem2_6_CA14F8B41F041609001400B79C32386E
        (:`NewEnumerator1`
          (return "NewEnumerator0"))
        (:`NewEnumerator2`
          _)
        (:`NewEnumerator3`
          (return "NewEnumerator7"))
        (:`NewEnumerator4`
          (return "NewEnumerator9"))))
    (:`NewEnumerator2`
      (switch `/Game/Blueprints/Enums/ENUM_Elem` InputCombination_Elem2_6_CA14F8B41F041609001400B79C32386E
        (:`NewEnumerator1`
          _)
        (:`NewEnumerator2`
          (return "NewEnumerator2"))
        (:`NewEnumerator3`
          (return "NewEnumerator8"))
        (:`NewEnumerator4`
          (return "NewEnumerator3"))))
    (:`NewEnumerator3`
      (switch `/Game/Blueprints/Enums/ENUM_Elem` InputCombination_Elem2_6_CA14F8B41F041609001400B79C32386E
        (:`NewEnumerator1`
          (return "NewEnumerator7"))
        (:`NewEnumerator2`
          (return "NewEnumerator2"))
        (:`NewEnumerator3`
          (return "NewEnumerator6"))
        (:`NewEnumerator4`
          (return "NewEnumerator5"))))
    (:`NewEnumerator4`
      (switch `/Game/Blueprints/Enums/ENUM_Elem` InputCombination_Elem2_6_CA14F8B41F041609001400B79C32386E
        (:`NewEnumerator1`
          (return "NewEnumerator9"))
        (:`NewEnumerator2`
          (return "NewEnumerator3"))
        (:`NewEnumerator3`
          (return "NewEnumerator5"))
        (:`NewEnumerator4`
          (return "NewEnumerator4")))))
  (return "NewEnumerator1"))

(fn `UserConstructionScript`)