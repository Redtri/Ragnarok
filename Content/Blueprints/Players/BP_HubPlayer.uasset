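; BP_HubPlayer is the Paper2D hub player character, which walks around and exits into the next level.
; Axis input moves it, picks idle or walk flipbooks and repositions its interact trigger, while Tick rescales the sprite per animation.
; Attack in the Exit state shows a loading screen and opens the level named from GM_MainMenu's influence.
; Attack and build functions are disconnected; element-to-tower and audio-channel helpers remain.
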(event `self.ReceiveBeginPlay`
  ;[1 1 1] Init
  (`self.Init`))

(event `Init`
  ;[1 1 1] Init
  (`self.InitializeProperties`))

(event `InputAxis|MoveForward`
  (params (AxisValue :type "Float (single-precision)"))
  (bind _returnvalue (> AxisValue 0.2))
  (bind _interacttrigger (`self.InteractTrigger`))
  (bind _paperflipbook (`self.PaperFlipbook`))
  (bind _m_animations (`self.M Animations`))
  ;[1 0.1788 0] Moving controls
  (if (and (not false) (not false))
    (if (or (or _returnvalue (< AxisValue -0.2)) (or (< (stale `InputAxis|MoveRight` AxisValue) -0.2) (> (stale `InputAxis|MoveRight` AxisValue) 0.2)))
      (`self.AddMovementInput` (`SceneComponent.GetForwardVector` (`self.Mesh`)) (* (`self.Speed`) AxisValue))
      (if _returnvalue
        ;;[1 1 1] Applies TEUB transform
        (`SceneComponent.K2_SetRelativeLocation` _interacttrigger (515.0 -30.0 0.0) false false)
        (`SceneComponent.K2_SetRelativeRotation` :`self` _interacttrigger :!label _label)
        (if (> AxisValue (`KismetMathLibrary.Abs` (stale `InputAxis|MoveRight` AxisValue))) :!label _label_2
          (`PaperFlipbookComponent.SetFlipbook` _paperflipbook (`|GetArrayItem` _m_animations (`self.INDEX_MoveFront`)))
          (else
            (`PaperFlipbookComponent.SetFlipbook` _paperflipbook (`|GetArrayItem` _m_animations (`self.INDEX_MoveSide`)))))
        (elif (< AxisValue -0.2)
          (`SceneComponent.K2_SetRelativeLocation` _interacttrigger (-515.0 -30.0 0.0) false false)
          (goto _label)))
      (else
        (`PaperFlipbookComponent.SetFlipbook` (`self.PaperFlipbook`) (`|GetArrayItem` (`self.M Animations`) (`self.INDEX_IdleFront`)) :!label _label_3)))))

(event `InputAxis|MoveRight`
  (params (AxisValue :type "Float (single-precision)"))
  (bind _returnvalue (> AxisValue 0.2))
  (bind _interacttrigger (`self.InteractTrigger`))
  (bind _paperflipbook (`self.PaperFlipbook`))
  ;[1 0.1788 0] Moving controls
  (if (and (not false) (not false))
    (if (or (or (> (stale `InputAxis|MoveForward` AxisValue) 0.2) (< (stale `InputAxis|MoveForward` AxisValue) -0.2)) (or (< AxisValue -0.2) _returnvalue))
      (`self.AddMovementInput` (`SceneComponent.GetRightVector` (`self.Mesh`)) (* (`self.Speed`) AxisValue))
      (if _returnvalue
        (`SceneComponent.K2_SetRelativeRotation` _paperflipbook (struct :`Yaw` -90.0 :`Roll` 90.0) false false)
        ;;[1 1 1] Applies TEUB transform
        (`SceneComponent.K2_SetRelativeLocation` _interacttrigger (50.0 370.0 0.0) false false)
        (`SceneComponent.K2_SetRelativeRotation` _interacttrigger (struct :`Yaw` 90.0) false false :!label _label_4)
        (goto _label_2)
        (elif (< AxisValue -0.2)
          (`SceneComponent.K2_SetRelativeRotation` _paperflipbook (struct :`Pitch` 180.0 :`Yaw` -90.0 :`Roll` 90.0) false false)
          (`SceneComponent.K2_SetRelativeLocation` _interacttrigger (50.0 -430.0 0.0) false false)
          (goto _label_4)))
      (else
        (goto _label_3)))))

(event `self.ReceiveTick`
  (params (DeltaSeconds :type "Float (single-precision)"))
  (bind _returnvalue (`PaperFlipbookComponent.GetFlipbook` (`self.PaperFlipbook`)))
  ;[1 1 1] Scaling up the WONDERFUL GRAPHISTS WORK
  (`SceneComponent.SetWorldScale3D` (`self.PaperFlipbook`) (select `bool` (or (== (`|GetArrayItem` (`self.M Animations`) (`self.INDEX_MoveFront`)) _returnvalue) (== _returnvalue (`|GetArrayItem` (`self.M Animations`) (`self.INDEX_Attack`)))) :`false` (0.5 0.5 0.5) :`true` (1.0 1.0 1.0) :!type "Vector Structure")))

(event `InputAction|Attack`
  (params (Key :type "Key Structure"))
  (bind _m_levelinfluence (`/Game/Blueprints/Gamemodes/GM_MainMenu.M LevelInfluence` (`self.M GameModeRef`)))
  ;[1 1 1] Reacts considering the player state
  (:`Pressed`
    (switch `/Game/Blueprints/Enums/ENUM_HubStates` (`self.M CurrentState`)
      (:`NewEnumerator1`
        (bind _returnvalue (`|CreateWidget` "/Game/Blueprints/Widgets/HUB/WBP_LoadingScreen.WBP_LoadingScreen_C" (`GameplayStatics.GetPlayerController` 0)))
        (`UserWidget.AddToViewport` _returnvalue 0)
        (`GameplayStatics.OpenLevel` (`KismetStringLibrary.Conv_StringToName` (`KismetStringLibrary.Concat_StrStr` "Level_" (`KismetStringLibrary.Conv_NameToString` (select `bool` (`|EnumEquality` _m_levelinfluence "NewEnumerator0") :`false` (`KismetStringLibrary.Conv_StringToName` (`|GetEnumeratorNameAsString` _m_levelinfluence)) :`true` "Neutral")))))))))

(fn `Attack`)

(fn `BuildTower`)

(fn `GetFreeActionChannel`
  (returns (Channel :type "AudioComponent Object Reference"))
  (bind _channel_action (`self.Channel_Action`))
  (bind _channel_action_01 (`self.Channel_Action_01`))
  (if (`AudioComponent.IsPlaying` _channel_action)
    (if (`AudioComponent.IsPlaying` _channel_action_01)
      (return _channel_action_01)
      (else
        (return null)))
    (else
      (return _channel_action))))

(fn `GetFreeMovementChannel`
  (returns (AudioSource :type "AudioComponent Object Reference"))
  (bind _channel_movement (`self.Channel_Movement`))
  (bind _channel_movement_01 (`self.Channel_Movement_01`))
  (bind _channel_movement_02 (`self.Channel_Movement_02`))
  (if (`AudioComponent.IsPlaying` _channel_movement)
    (if (`AudioComponent.IsPlaying` _channel_movement_01)
      (if (`AudioComponent.IsPlaying` _channel_movement_02)
        (return null)
        (else
          (return _channel_movement_02)))
      (else
        (return _channel_movement_01)))
    (else
      (return _channel_movement))))

(fn `GetRandomSoundFrom`
  (params (Sounds :type "Array of SoundWave Object Reference"))
  (returns (Return :type "SoundWave Object Reference"))
  (return (`|GetArrayItem` Sounds (`KismetMathLibrary.RandomIntegerInRange` 0 (- (`KismetArrayLibrary.Array_Length` Sounds) 1)))))

(fn `InitializeProperties`
  (locals (SoundArray :type "Array of SoundWave Object Reference"))
  (bind _m_animations (`self.M Animations`))
  ;[1 1 1] Animations
  (`KismetArrayLibrary.Array_Add` _m_animations "/Game/Sprites/Flipbooks/Player/Player_FrontIdle.Player_FrontIdle")
  (`KismetArrayLibrary.Array_Add` _m_animations "/Game/Sprites/Flipbooks/Player/Player_SideIdle.Player_SideIdle")
  (`KismetArrayLibrary.Array_Add` _m_animations "/Game/Sprites/Flipbooks/Player/Player_BackWalk.Player_BackWalk")
  (`KismetArrayLibrary.Array_Add` _m_animations "/Game/Sprites/Flipbooks/Player/Player_SideWalk.Player_SideWalk")
  (`KismetArrayLibrary.Array_Add` _m_animations "/Game/Sprites/Flipbooks/Player/Player_SideAttack.Player_SideAttack")
  (`KismetArrayLibrary.Array_Add` _m_animations "/Game/Sprites/Flipbooks/Player/Player_Building.Player_Building")
  ;[1 1 1] References
  (set `self.M GameModeRef` (cast `/Game/Blueprints/Gamemodes/GM_MainMenu` (`GameplayStatics.GetGameMode`) :!pure true)))

(fn `InputToTower`
  (params (InputCombination :type "/Game/Blueprints/Structs/STRUCT_ElemToTowers Structure"))
  (returns (TowerType :type "/Game/Blueprints/Enums/ENUM_TowerType Enum"))
  (switch `/Game/Blueprints/Enums/ENUM_Elem` InputCombination_Elem1_4_C9F7FD3328041609000E00D28746D39E
    (:`NewEnumerator1`
      (switch `/Game/Blueprints/Enums/ENUM_Elem` InputCombination_Elem2_6_CA14F8B41F041609001400B79C32386E
        (:`NewEnumerator1`
          (return "NewEnumerator0"))
        (:`NewEnumerator2`
          _)
        (:`NewEnumerator3`
          (return "NewEnumerator7"))
        (:`NewEnumerator4`
          (return "NewEnumerator9"))))
    (:`NewEnumerator2`
      (switch `/Game/Blueprints/Enums/ENUM_Elem` InputCombination_Elem2_6_CA14F8B41F041609001400B79C32386E
        (:`NewEnumerator1`
          _)
        (:`NewEnumerator2`
          (return "NewEnumerator2"))
        (:`NewEnumerator3`
          (return "NewEnumerator8"))
        (:`NewEnumerator4`
          (return "NewEnumerator3"))))
    (:`NewEnumerator3`
      (switch `/Game/Blueprints/Enums/ENUM_Elem` InputCombination_Elem2_6_CA14F8B41F041609001400B79C32386E
        (:`NewEnumerator1`
          (return "NewEnumerator7"))
        (:`NewEnumerator2`
          (return "NewEnumerator2"))
        (:`NewEnumerator3`
          (return "NewEnumerator6"))
        (:`NewEnumerator4`
          (return "NewEnumerator5"))))
    (:`NewEnumerator4`
      (switch `/Game/Blueprints/Enums/ENUM_Elem` InputCombination_Elem2_6_CA14F8B41F041609001400B79C32386E
        (:`NewEnumerator1`
          (return "NewEnumerator9"))
        (:`NewEnumerator2`
          (return "NewEnumerator3"))
        (:`NewEnumerator3`
          (return "NewEnumerator5"))
        (:`NewEnumerator4`
          (return "NewEnumerator4")))))
  (return "NewEnumerator1"))

(fn `UserConstructionScript`)