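; Play-mode game mode for an elemental rat-defense game, running ambient audio, rat hordes, score and HUB damage.
; Setup loads game-instance state and BP_STD tables, then skins props by current element.
; Hordes spawn recursively at random points through a delay-tolerant loop macro, upgrading the rat type matching that element.
; Once all rats are gone, the element with most accumulated tower damage becomes the saved influence and the goal appears.
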(event `self.ReceiveBeginPlay`
  (bind _track_ambient02 (`self.Track_Ambient02`))
  (bind _track_ambient03 (`self.Track_Ambient03`))
  (bind _track_event (`self.Track_Event`))
  (bind _track_ambient01 (`self.Track_Ambient01`))
  (bind _track_other (`self.Track_Other`))
  ;[1 1 1] Init
  (`/Game/Blueprints/Players/BP_Player.Init` (cast `/Game/Blueprints/Players/BP_Player` (`GameplayStatics.GetPlayerCharacter` 0) :!pure true))
  (`self.Init`)
  (`AudioComponent.SetSound` _track_other "/Game/Sounds/Ambiances/Classic/Ambiance-Neutre-Paisible.Ambiance-Neutre-Paisible")
  (`AudioComponent.Play` _track_other 0.0)
  (`KismetSystemLibrary.Delay` 10.0)
  (`AudioComponent.SetSound` _track_ambient01 "/Game/Sounds/Ambiances/Classic/Ambiance-Neutre-General_Cue.Ambiance-Neutre-General_Cue")
  (`AudioComponent.Play` _track_ambient01 0.0)
  (`AudioComponent.FadeIn` _track_ambient01 10.0 1.0 0.0)
  (`AudioComponent.SetSound` _track_ambient02 "/Game/Sounds/Ambiances/Classic/Ambiance-Neutre-Thunder-1_Cue.Ambiance-Neutre-Thunder-1_Cue")
  (`AudioComponent.Play` _track_ambient02 0.0)
  (`AudioComponent.FadeIn` _track_ambient02 10.0 1.0 0.0)
  (`AudioComponent.SetSound` _track_ambient03 "/Game/Sounds/Ambiances/Classic/Ambiance-Neutre-Thunder-2_Cue.Ambiance-Neutre-Thunder-2_Cue")
  (`AudioComponent.Play` _track_ambient03 0.0)
  (`AudioComponent.FadeIn` _track_ambient03 10.0 1.0 0.0)
  (`KismetSystemLibrary.Delay` 5.0)
  (`AudioComponent.SetSound` _track_event "/Game/Sounds/Ambiances/Classic/Ambiance-Bell-Fast.Ambiance-Bell-Fast")
  (`AudioComponent.Play` _track_event 0.0)
  (`KismetSystemLibrary.Delay` 5.0)
  (`AudioComponent.FadeOut` (`self.Track_Other`) 20.0 0.0)
  (`KismetSystemLibrary.PrintString` "Calling next horde")
  ;[1 1 1] Spawner
  (`self.SpawnNextHordes`))

(event `SpawnNextWave`
  ;[1 1 1] Spawner
  (`self.SpawnNextHordes`))

(event `Init`
  ;[1 1 1] Init
  (`KismetSystemLibrary.Delay` 0.2)
  (`self.InitializeProperties`))

(event `SpawnNextHordes`
  (bind _m_levelinfluence (`self.M LevelInfluence`))
  (bind _value (`BlueprintMapLibrary.Map_Find` (`self.M WavesSTD`) (`self.M LevelInfluence`)))
  (bind (_output_rattype _output_size _output_spawnrate) (break `/Game/Blueprints/Structs/STRUCT_Horde` (`|GetArrayItem` (break `/Game/Blueprints/Structs/STRUCT_Wave` _value) (`self.M CurrentHordeIndex`))))
  ;[1 1 1] Spawner
  ;;[1 1 1] For each number of a same horde
  (`self.PermissiveForLoop` 0 (- _output_size 1) :!label _label
    (:`Loop Body`
      (set `self.M CurrentSpawnPtIndex` (`KismetMathLibrary.RandomIntegerInRange` 0 (- (`KismetArrayLibrary.Array_Length` (`self.M RatSpawnPoints`)) 1)))
      (`KismetSystemLibrary.Delay` (`.HordeSpawnDelay_21_4E5BDAC74042EFDBEEA7A7BEE6A555FA` (break `/Game/Blueprints/Structs/STRUCT_Wave` _value)))
      (set `self.M AssaultStarted` true)
      ;;[1 1 1] Spawns rats
      (`self.PermissiveForLoop` 0 (- (`BlueprintMapLibrary.Map_Find` (`self.M HordesSTD`) _output_rattype) 1) :!label _label_2
        (:`Loop Body`
          (`KismetSystemLibrary.Delay` _output_spawnrate)
          (bind _ratreference (`/Game/Blueprints/Actors/GameplayElement/BP_RatSpawnPoint.SpawnRatType` (`|GetArrayItem` (`self.M RatSpawnPoints`) (`self.M CurrentSpawnPtIndex`)) _output_rattype (select `/Game/Blueprints/Enums/ENUM_RatType` _output_rattype :`NewEnumerator1` (`|EnumEquality` _m_levelinfluence "NewEnumerator4") :`NewEnumerator6` (`|EnumEquality` _m_levelinfluence "NewEnumerator3") :`NewEnumerator2` (`|EnumEquality` _m_levelinfluence "NewEnumerator1") :`NewEnumerator3` (`|EnumEquality` _m_levelinfluence "NewEnumerator2"))))
          (`KismetArrayLibrary.Array_Add` (`self.M SpawnedRats`) _ratreference)
          (goto _label_2 :!via `NextStepIn`))
        (:`Completed`
          (goto _label :!via `NextStepIn`))))
    (:`Completed`
      (if (< (`self.M CurrentHordeIndex`) (`KismetArrayLibrary.Array_Length` (break `/Game/Blueprints/Structs/STRUCT_Wave` _value)))
        (`/Engine/EditorBlueprintResources/StandardMacros.IncrementInt` (`self.M CurrentHordeIndex`)
          (:`  `
            (`self.SpawnNextHordes`)))
        (else
          (set `self.M CurrentHordeIndex` 0)
          (set `self.M LastWaveSent` true)
          (`KismetSystemLibrary.PrintString` "Last wave sent"))))))

(event `self.ReceiveTick`
  (params (DeltaSeconds :type "Float (single-precision)"))
  (bind _m_levelinfluence (`self.M LevelInfluence`))
  (bind (_m_gamedata_lives _m_gamedata_score _m_gamedata_nbwaves) (break `/Game/Blueprints/Structs/STRUCT_GameData` (`self.M GameData`)))
  ;[1 1 1] Checks for the current assault state
  (if (and (`self.M LastWaveSent`) (`self.M AssaultStarted`) (not (`self.M AssaultCleared`)) (== (`KismetArrayLibrary.Array_Length` (`self.M SpawnedRats`)) 0))
    ;;[1 0 0.006649] Watch out struct incrementation
    (set `self.M AssaultCleared` true)
    (`/Engine/EditorBlueprintResources/StandardMacros.IncrementInt` _m_gamedata_nbwaves
      (:`  `
        (`/Game/Blueprints/Actors/GameplayElement/BP_Goal.SetGameData` (`self.M GoalRef`) (`self.M GameData`))
        (switch `int` (`KismetMathLibrary.MaxOfFloatArray` (`|MakeArray` (`self.M WindTotal`) (`self.M FireTotal`) (`self.M WaterTotal`) (`self.M EarthTotal`)))
          (:`0`
            (set `self.M LevelInfluence` "NewEnumerator2"))
          (:`1`
            (set `self.M LevelInfluence` "NewEnumerator1"))
          (:`2`
            (set `self.M LevelInfluence` "NewEnumerator4"))
          (:`3`
            (set `self.M LevelInfluence` "NewEnumerator3")))
        (`self.UpdateGameInstanceData` (`self.M GameData`) _m_levelinfluence)
        (`KismetSystemLibrary.PrintString` (`|GetEnumeratorNameAsString` _m_levelinfluence))
        ;[1 1 1] Spawn some signage for the player to go back into the HUB
        (`KismetSystemLibrary.PrintString` (`KismetStringLibrary.Concat_StrStr` "Assault clear : " "Wind : " (`KismetStringLibrary.Conv_DoubleToString` (`self.M WindTotal`)) ". Fire : " (`KismetStringLibrary.Conv_DoubleToString` (`self.M FireTotal`)) ". Water : " (`KismetStringLibrary.Conv_DoubleToString` (`self.M WaterTotal`)) ". Earth : " (`KismetStringLibrary.Conv_DoubleToString` (`self.M EarthTotal`))))
        (`/Game/Blueprints/Actors/GameplayElement/BP_Goal.Appearing` (`self.M GoalRef`))))))

(event `RemoveRat`
  (params (Rat :type "/Game/Blueprints/Actors/Enemy/BP_BaseRat Object Reference") (Killed :type Boolean))
  (bind (_m_rattype_type _m_rattype_iscc _m_rattype_element _m_rattype_hp _m_rattype_speed _m_rattype_damage) (break `/Game/Blueprints/Structs/STRUCT_Rat` (`/Game/Blueprints/Actors/Enemy/BP_BaseRat.M RatType` Rat)))
  (bind _m_hub_goal (`self.M HUB_Goal`))
  (bind (_m_gamedata_lives _m_gamedata_score) (break `/Game/Blueprints/Structs/STRUCT_GameData` (`self.M GameData`)))
  ;[1 1 1] Spawner
  ;;[1 1 1] Removes rats
  (`KismetArrayLibrary.Array_RemoveItem` (`self.M SpawnedRats`) Rat)
  (if Killed
    (`/Engine/EditorBlueprintResources/StandardMacros.IncrementInt` _m_gamedata_score
      (:`  `
        (`/Game/Blueprints/Actors/GameplayElement/BP_Goal.SetGameData` (`self.M GoalRef`) (`self.M GameData`))))
    (else
      ;;;[0 0 0] HUB health decrease
      (`/Game/Blueprints/Actors/GameplayElement/BP_HUB.LowerHealth` _m_hub_goal (/ _m_rattype_damage (`self.CONST_MaxHealthHUB`)))
      (bind _object (`/Game/Blueprints/Actors/GameplayElement/BP_HUB.GetHealthBar` _m_hub_goal))
      (`/Game/Blueprints/Widgets/HealthBars/WBP_HUB_HealthBar.RefreshHpLoss` _object (`KismetMathLibrary.FTrunc` _m_rattype_damage)))))

(fn `AddDamagesFromTower`
  (params (TowerInfos :type "/Game/Blueprints/Structs/STRUCT_Tower Structure") (DamagesAmount :type "Float (double-precision)"))
  (if (`|EnumEquality` TowerInfos_Elem1_11_6F7333C84422AFB39DDC2583DEEED404 TowerInfos_Elem2_12_2DE741FC446D3A375FB82982600E57E9)
    (`self.AddElementalDamages` TowerInfos_Elem1_11_6F7333C84422AFB39DDC2583DEEED404 DamagesAmount)
    (else
      (`self.AddElementalDamages` TowerInfos_Elem1_11_6F7333C84422AFB39DDC2583DEEED404 DamagesAmount)
      (`self.AddElementalDamages` TowerInfos_Elem2_12_2DE741FC446D3A375FB82982600E57E9 DamagesAmount))))

(fn `AddElementalDamages`
  (params (Element :type "/Game/Blueprints/Enums/ENUM_Elem Enum" :default "NewEnumerator0") (DamagesAmount :type "Float (double-precision)"))
  (switch `/Game/Blueprints/Enums/ENUM_Elem` Element
    (:`NewEnumerator1`
      (set `self.M FireTotal` (+ (`self.M FireTotal`) DamagesAmount)))
    (:`NewEnumerator2`
      (set `self.M WindTotal` (+ (`self.M WindTotal`) DamagesAmount)))
    (:`NewEnumerator3`
      (set `self.M EarthTotal` (+ (`self.M EarthTotal`) DamagesAmount)))
    (:`NewEnumerator4`
      (set `self.M WaterTotal` (+ (`self.M WaterTotal`) DamagesAmount)))))

(fn `GetRandomRat`
  (returns (Return :type "/Game/Blueprints/Enums/ENUM_RatType Enum"))
  (bind _m_ratstd (`self.M RatSTD`))
  (bind _values (`BlueprintMapLibrary.Map_Values` _m_ratstd))
  (bind _output_type (break `/Game/Blueprints/Structs/STRUCT_Rat` (`|GetArrayItem` _values (`KismetMathLibrary.RandomIntegerInRange` 0 (- (`BlueprintMapLibrary.Map_Length` _m_ratstd) 1)))))
  (return _output_type))

(fn `InitializeProperties`
  ;[1 1 1] State values
  (bind _asbp_game_instance (cast `/Game/Blueprints/GameInstances/BP_GameInstance` (`GameplayStatics.GetGameInstance`)))
  (set `self.M LevelInfluence` (`/Game/Blueprints/GameInstances/BP_GameInstance.M LevelInfluence` _asbp_game_instance))
  (set `self.M GameData` (`/Game/Blueprints/GameInstances/BP_GameInstance.M GameData` _asbp_game_instance))
  (set `self.M CurrentHordeIndex` 0)
  ;[1 1 1] Sets STD values from STD container
  (bind _outactors (`GameplayStatics.GetAllActorsOfClass` "/Game/Blueprints/Abstract/BP_STD.BP_STD_C"))
  (bind _output (`|GetArrayItem` _outactors))
  (set `self.M TowerSTD` (`/Game/Blueprints/Abstract/BP_STD.M TowerSTD` _output))
  (set `self.M RatSTD` (`/Game/Blueprints/Abstract/BP_STD.M RatSTD` _output))
  (set `self.M RatSTDSpawnSounds` (`/Game/Blueprints/Abstract/BP_STD.M RatSTDSpawnSounds` _output))
  (set `self.M HordesSTD` (`/Game/Blueprints/Abstract/BP_STD.M HordesSTD` _output))
  (set `self.M WavesSTD` (`/Game/Blueprints/Abstract/BP_STD.M WavesSTD` _output))
  ;[1 1 1] References Rat spawn points
  (bind _outactors_2 (`GameplayStatics.GetAllActorsOfClass` "/Game/Blueprints/Actors/GameplayElement/BP_RatSpawnPoint.BP_RatSpawnPoint_C"))
  (set `self.M RatSpawnPoints` _outactors_2)
  ;[1 1 1] References Game Instance
  (bind _asbp_game_instance_2 (cast `/Game/Blueprints/GameInstances/BP_GameInstance` (`GameplayStatics.GetGameInstance`)))
  (set `self.M GameInstanceRef` _asbp_game_instance_2)
  ;[1 1 1] Initializes BP_Goal infos
  (`self.SetGameData` (`/Game/Blueprints/GameInstances/BP_GameInstance.M GameData` (`self.M GameInstanceRef`)))
  (bind _outactors_3 (`GameplayStatics.GetAllActorsOfClass` "/Game/Blueprints/Actors/GameplayElement/BP_Goal.BP_Goal_C"))
  (bind _output_get (set `self.M GoalRef` (`|GetArrayItem` _outactors_3)))
  (`/Game/Blueprints/Actors/GameplayElement/BP_Goal.SetGameData` _output_get (`self.M GameData`))
  (bind _outactors_4 (`GameplayStatics.GetAllActorsOfClass` "/Game/Blueprints/Actors/GameplayElement/BP_HUB.BP_HUB_C"))
  (bind _output_get_2 (set `self.M HUB_Goal` (`|GetArrayItem` _outactors_4)))
  (`/Game/Blueprints/Actors/GameplayElement/BP_HUB.SetHealth` _output_get_2 1.0)
  ;[1 1 1] Environment appearance
  (bind _outactors_5 (`GameplayStatics.GetAllActorsOfClass` "/Game/Blueprints/Actors/Props/BP_PropBase.BP_PropBase_C"))
  (for _array_element _outactors_5
    (`/Game/Blueprints/Actors/Props/BP_PropBase.UpdateSkin` _array_element (`self.M LevelInfluence`))))

(fn `SetGameData`
  (params (Data :type "/Game/Blueprints/Structs/STRUCT_GameData Structure"))
  (set `self.M GameData` Data))

(fn `UpdateGameInstanceData`
  (params (Data :type "/Game/Blueprints/Structs/STRUCT_GameData Structure") (LevelInfluence :type "/Game/Blueprints/Enums/ENUM_Elem Enum" :default "NewEnumerator0"))
  (`/Game/Blueprints/GameInstances/BP_GameInstance.UpdateData` (`self.M GameInstanceRef`) Data LevelInfluence))

(fn `UserConstructionScript`)