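; BP_STD is a sound data Blueprint that holds rat spawn intro sounds and player movement and attack sounds.
; Its Construction Script fills a map of rat intros keyed by type name, with "Up" keys for elemental Tank, Speed, Ninja and Flying variants.
; A scratch array is refilled and cleared for each map entry.
; Player footstep and attack sounds go into two separate arrays.
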(fn `UserConstructionScript`
  (locals (SoundArray :type "Array of SoundWave Object Reference"))
  (bind _soundarray (`local.SoundArray`))
  (bind _soundarray_2 (`local.SoundArray`))
  (bind _soundarray_3 (`local.SoundArray`))
  (bind _soundarray_4 (`local.SoundArray`))
  (bind _m_playermovesounds (`self.M PlayerMoveSounds`))
  (bind _m_playerattacksounds (`self.M PlayerAttackSounds`))
  (bind _soundarray_5 (`local.SoundArray`))
  (bind _soundarray_6 (`local.SoundArray`))
  (bind _soundarray_7 (`local.SoundArray`))
  (bind _soundarray_8 (`local.SoundArray`))
  (bind _soundarray_9 (`local.SoundArray`))
  ;[1 1 1] Rat spawn sounds
  ;;[1 1 1] Grunt
  (`KismetArrayLibrary.Array_Add` _soundarray "/Game/Sounds/Rat_sounds/Grunt/Rat-Grunt-Intro-1.Rat-Grunt-Intro-1")
  (`KismetArrayLibrary.Array_Add` _soundarray "/Game/Sounds/Rat_sounds/Grunt/Rat-Grunt-Intro-2.Rat-Grunt-Intro-2")
  (`BlueprintMapLibrary.Map_Add` (`self.M RatSTDSpawnSounds`) "Grunt" (make `/Game/Blueprints/Structs/STRUCT_AudioContainer` _soundarray))
  (`KismetArrayLibrary.Array_Clear` _soundarray)
  ;;[1 1 1] Tank
  (`KismetArrayLibrary.Array_Add` _soundarray_6 "/Game/Sounds/Rat_Sound_-_Tank/Tank/Rat-Tank-Intro-1.Rat-Tank-Intro-1")
  (`KismetArrayLibrary.Array_Add` _soundarray_6 "/Game/Sounds/Rat_Sound_-_Tank/Tank/Rat-Tank-Intro-2.Rat-Tank-Intro-2")
  (`BlueprintMapLibrary.Map_Add` (`self.M RatSTDSpawnSounds`) "Tank" (make `/Game/Blueprints/Structs/STRUCT_AudioContainer` _soundarray_6))
  (`KismetArrayLibrary.Array_Clear` _soundarray_6)
  (`KismetArrayLibrary.Array_Add` _soundarray_8 "/Game/Sounds/Rat_Sound_-_Tank/Tank/Rat-Tank-Earth-Intro-1.Rat-Tank-Earth-Intro-1")
  (`KismetArrayLibrary.Array_Add` _soundarray_8 "/Game/Sounds/Rat_Sound_-_Tank/Tank/Rat-Tank-Earth-Intro-2.Rat-Tank-Earth-Intro-2")
  (`BlueprintMapLibrary.Map_Add` (`self.M RatSTDSpawnSounds`) "TankUp" (make `/Game/Blueprints/Structs/STRUCT_AudioContainer` _soundarray_8))
  (`KismetArrayLibrary.Array_Clear` _soundarray_8)
  ;;[1 1 1] Speed
  (`KismetArrayLibrary.Array_Add` _soundarray_9 "/Game/Sounds/Rat_sounds/Speed_Rat/Rat-Speedrat-Intro-1.Rat-Speedrat-Intro-1")
  (`KismetArrayLibrary.Array_Add` _soundarray_9 "/Game/Sounds/Rat_sounds/Speed_Rat/Rat-Speedrat-Intro-2.Rat-Speedrat-Intro-2")
  (`KismetArrayLibrary.Array_Add` _soundarray_9 "/Game/Sounds/Rat_sounds/Speed_Rat/Rat-Speedrat-Intro-3.Rat-Speedrat-Intro-3")
  (`BlueprintMapLibrary.Map_Add` (`self.M RatSTDSpawnSounds`) "Speed" (make `/Game/Blueprints/Structs/STRUCT_AudioContainer` _soundarray_9))
  (`KismetArrayLibrary.Array_Clear` _soundarray_9)
  (`KismetArrayLibrary.Array_Add` _soundarray_2 "/Game/Sounds/Rat_sounds/Speed_Rat/Rat-Speedrat-Fire-Intro-1.Rat-Speedrat-Fire-Intro-1")
  (`KismetArrayLibrary.Array_Add` _soundarray_2 "/Game/Sounds/Rat_sounds/Speed_Rat/Rat-Speedrat-Fire-Intro-2.Rat-Speedrat-Fire-Intro-2")
  (`KismetArrayLibrary.Array_Add` _soundarray_2 "/Game/Sounds/Rat_sounds/Speed_Rat/Rat-Speedrat-Fire-Intro-3.Rat-Speedrat-Fire-Intro-3")
  (`BlueprintMapLibrary.Map_Add` (`self.M RatSTDSpawnSounds`) "SpeedUp" (make `/Game/Blueprints/Structs/STRUCT_AudioContainer` _soundarray_2))
  (`KismetArrayLibrary.Array_Clear` _soundarray_2)
  ;;[1 1 1] Ninja
  (`KismetArrayLibrary.Array_Add` _soundarray_3 "/Game/Sounds/Ninja/Ninja/Rat-Ninja-Intro-1.Rat-Ninja-Intro-1")
  (`KismetArrayLibrary.Array_Add` _soundarray_3 "/Game/Sounds/Ninja/Ninja/Rat-Ninja-Intro-2.Rat-Ninja-Intro-2")
  (`BlueprintMapLibrary.Map_Add` (`self.M RatSTDSpawnSounds`) "Ninja" (make `/Game/Blueprints/Structs/STRUCT_AudioContainer` _soundarray_3))
  (`KismetArrayLibrary.Array_Clear` _soundarray_3)
  (`KismetArrayLibrary.Array_Add` _soundarray_4 "/Game/Sounds/Ninja/Ninja/Rat-Ninja-Wind-Intro-1.Rat-Ninja-Wind-Intro-1")
  (`KismetArrayLibrary.Array_Add` _soundarray_4 "/Game/Sounds/Ninja/Ninja/Rat-Ninja-Wind-Intro-2.Rat-Ninja-Wind-Intro-2")
  (`BlueprintMapLibrary.Map_Add` (`self.M RatSTDSpawnSounds`) "NinjaUp" (make `/Game/Blueprints/Structs/STRUCT_AudioContainer` _soundarray_4))
  (`KismetArrayLibrary.Array_Clear` _soundarray_4)
  ;;[1 1 1] Flying
  (`KismetArrayLibrary.Array_Add` _soundarray_5 "/Game/Sounds/Rat_sounds/Flying_Rat/Rat-Flyingrat-Intro-1.Rat-Flyingrat-Intro-1")
  (`KismetArrayLibrary.Array_Add` _soundarray_5 "/Game/Sounds/Rat_sounds/Flying_Rat/Rat-Flyingrat-Intro-2.Rat-Flyingrat-Intro-2")
  (`BlueprintMapLibrary.Map_Add` (`self.M RatSTDSpawnSounds`) "Flying" (make `/Game/Blueprints/Structs/STRUCT_AudioContainer` _soundarray_5))
  (`KismetArrayLibrary.Array_Clear` _soundarray_5)
  (`KismetArrayLibrary.Array_Add` _soundarray_7 "/Game/Sounds/Rat_sounds/Flying_Rat/Rat-Flyingrat-Water-Intro-1.Rat-Flyingrat-Water-Intro-1")
  (`KismetArrayLibrary.Array_Add` _soundarray_7 "/Game/Sounds/Rat_sounds/Flying_Rat/Rat-Flyingrat-Water-Intro-2.Rat-Flyingrat-Water-Intro-2")
  (`BlueprintMapLibrary.Map_Add` (`self.M RatSTDSpawnSounds`) "FlyingUp" (make `/Game/Blueprints/Structs/STRUCT_AudioContainer` _soundarray_7))
  (`KismetArrayLibrary.Array_Clear` _soundarray_7)
  ;[1 1 1] Player sounds
  (`KismetArrayLibrary.Array_Add` _m_playermovesounds "/Game/Sounds/Perso/Perso-Step-1.Perso-Step-1")
  (`KismetArrayLibrary.Array_Add` _m_playermovesounds "/Game/Sounds/Perso/Perso-Step-2.Perso-Step-2")
  (`KismetArrayLibrary.Array_Add` _m_playermovesounds "/Game/Sounds/Perso/Perso-Step-3.Perso-Step-3")
  (`KismetArrayLibrary.Array_Add` _m_playermovesounds "/Game/Sounds/Perso/Perso-Step-4.Perso-Step-4")
  (`KismetArrayLibrary.Array_Add` _m_playermovesounds "/Game/Sounds/Perso/Perso-Step-5.Perso-Step-5")
  (`KismetArrayLibrary.Array_Add` _m_playermovesounds "/Game/Sounds/Perso/Perso-Step-6.Perso-Step-6")
  (`KismetArrayLibrary.Array_Add` _m_playerattacksounds "/Game/Sounds/Perso/Perso-Attack-1.Perso-Attack-1")
  (`KismetArrayLibrary.Array_Add` _m_playerattacksounds "/Game/Sounds/Perso/Perso-Attack-2.Perso-Attack-2")
  (`KismetArrayLibrary.Array_Add` _m_playerattacksounds "/Game/Sounds/Perso/Perso-Attack-3.Perso-Attack-3")
  (`KismetArrayLibrary.Array_Add` _m_playerattacksounds "/Game/Sounds/Perso/Perso-Attack-4.Perso-Attack-4")
  (`KismetArrayLibrary.Array_Add` _m_playerattacksounds "/Game/Sounds/Perso/Perso-Attack-5.Perso-Attack-5")
  (`KismetArrayLibrary.Array_Add` _m_playerattacksounds "/Game/Sounds/Perso/Perso-Attack-6.Perso-Attack-6")
  (`KismetArrayLibrary.Array_Add` _m_playerattacksounds "/Game/Sounds/Perso/Perso-Attack-7.Perso-Attack-7"))