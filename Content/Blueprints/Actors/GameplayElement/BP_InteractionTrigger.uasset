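; Interaction trigger for a tower spot that shows the player's two-element input combination as crystal sprites.
; When a player overlaps it and the slot is free, it shows a lozenge and registers as the player's interactable; leaving hides it and clears the combination.
; FirstInput and SecondInput set the bottom and top triangle's sprite and position per element.
; The construction script hides both triangles and snaps the actor to its linked tower spot.
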(event `Display`
  (params (Show :type Boolean))
  ;[1 1 1] DISPLAY
  (`SceneComponent.SetVisibility` (`self.Losange`) Show false)
  (`SceneComponent.SetVisibility` (`self.Triangle1`) Show false)
  (`SceneComponent.SetVisibility` (`self.Triangle2`) Show false))

(event `self.Trigger.OnComponentBeginOverlap`
  (params (OverlappedComponent :type "PrimitiveComponent Object Reference") (OtherActor :type "Actor Object Reference") (OtherComp :type "PrimitiveComponent Object Reference") (OtherBodyIndex :type Integer) (bFromSweep :type Boolean) (SweepResult :type "HitResult Structure (by ref)"))
  ;[1 1 1] Show
  (bind _asbp_player (cast `/Game/Blueprints/Players/BP_Player` OtherActor))
  (if (`/Game/Blueprints/Actors/GameplayElement/BP_TowerSpawnPoint.M IsFreeSlot` (`self.M TowerSpot`))
    (`self.Display` true)
    (`SceneComponent.SetVisibility` (`self.Triangle1`) false false)
    (`SceneComponent.SetVisibility` (`self.Triangle2`) false false)
    (set `/Game/Blueprints/Players/BP_Player.M Interactable` self _asbp_player)
    (set `/Game/Blueprints/Players/BP_Player.M CanInteract` true _asbp_player)))

(event `self.Trigger.OnComponentEndOverlap`
  (params (OverlappedComponent :type "PrimitiveComponent Object Reference") (OtherActor :type "Actor Object Reference") (OtherComp :type "PrimitiveComponent Object Reference") (OtherBodyIndex :type Integer))
  ;[1 1 1] Hide
  (bind _asbp_player (cast `/Game/Blueprints/Players/BP_Player` OtherActor))
  (`self.Display` false)
  (set `/Game/Blueprints/Players/BP_Player.M CanInteract` false _asbp_player)
  (set `/Game/Blueprints/Players/BP_Player.InputCombination` (make `/Game/Blueprints/Structs/STRUCT_ElemToTowers` "NewEnumerator0") _asbp_player)
  (`SceneComponent.SetVisibility` (`self.Triangle1`) false false :!label _label)
  (`SceneComponent.SetVisibility` (`self.Triangle2`) false false))

(event `SecondInput`
  (params (`2ndInput` :type "/Game/Blueprints/Enums/ENUM_Elem Enum" :default "NewEnumerator0"))
  (bind _triangle1 (`self.Triangle1`))
  (bind _m_trianglepositions (`self.M TrianglePositions`))
  ;[1 1 1] Applies transform
  (if (`/Game/Blueprints/Actors/GameplayElement/BP_TowerSpawnPoint.M IsFreeSlot` (`self.M TowerSpot`))
    (switch `/Game/Blueprints/Enums/ENUM_Elem` `2ndInput`
      (:`NewEnumerator0`
        (goto _label))
      (:`NewEnumerator1`
        (`PaperSpriteComponent.SetSprite` _triangle1 "/Game/Textures/InputInteraction/Cristal_rouge_haut_Sprite.Cristal_Rouge_Haut_Sprite")
        (`SceneComponent.K2_SetRelativeLocation` _triangle1 (`|GetArrayItem` _m_trianglepositions 4) false false))
      (:`NewEnumerator2`
        (`PaperSpriteComponent.SetSprite` _triangle1 "/Game/Textures/InputInteraction/Cristal_jaune_haut_Sprite.Cristal_Jaune_Haut_Sprite")
        (`SceneComponent.K2_SetRelativeLocation` _triangle1 (`|GetArrayItem` _m_trianglepositions 5) false false))
      (:`NewEnumerator3`
        (`PaperSpriteComponent.SetSprite` _triangle1 "/Game/Textures/InputInteraction/Cristal_vert_haut_Sprite.Cristal_Vert_Haut_Sprite")
        (`SceneComponent.K2_SetRelativeLocation` _triangle1 (`|GetArrayItem` _m_trianglepositions 6) false false))
      (:`NewEnumerator4`
        (`PaperSpriteComponent.SetSprite` _triangle1 "/Game/Textures/InputInteraction/Cristal_bleu_haut_Sprite.Cristal_Bleu_Haut_Sprite")
        (`SceneComponent.K2_SetRelativeLocation` _triangle1 (`|GetArrayItem` _m_trianglepositions 7) false false)))
    (`SceneComponent.SetVisibility` (`self.Triangle1`) true false)))

(event `FirstInput`
  (params (`1stInput` :type "/Game/Blueprints/Enums/ENUM_Elem Enum" :default "NewEnumerator0"))
  (bind _m_trianglepositions (`self.M TrianglePositions`))
  (bind _triangle2 (`self.Triangle2`))
  ;[1 1 1] Applies transform
  (if (`/Game/Blueprints/Actors/GameplayElement/BP_TowerSpawnPoint.M IsFreeSlot` (`self.M TowerSpot`))
    (switch `/Game/Blueprints/Enums/ENUM_Elem` `1stInput`
      (:`NewEnumerator0`
        (goto _label))
      (:`NewEnumerator1`
        (`PaperSpriteComponent.SetSprite` _triangle2 "/Game/Textures/InputInteraction/Cristal_rouge_bas_Sprite.Cristal_Rouge_Bas_Sprite")
        (`SceneComponent.K2_SetRelativeLocation` _triangle2 (`|GetArrayItem` _m_trianglepositions) false false))
      (:`NewEnumerator2`
        (`PaperSpriteComponent.SetSprite` _triangle2 "/Game/Textures/InputInteraction/Cristal_jaune_bas_Sprite.Cristal_Jaune_Bas_Sprite")
        (`SceneComponent.K2_SetRelativeLocation` _triangle2 (`|GetArrayItem` _m_trianglepositions 1) false false))
      (:`NewEnumerator3`
        (`PaperSpriteComponent.SetSprite` _triangle2 "/Game/Textures/InputInteraction/Cristal_vert_bas_Sprite.Cristal_Vert_Bas_Sprite")
        (`SceneComponent.K2_SetRelativeLocation` _triangle2 (`|GetArrayItem` _m_trianglepositions 2) false false))
      (:`NewEnumerator4`
        (`PaperSpriteComponent.SetSprite` _triangle2 "/Game/Textures/InputInteraction/Cristal_bleu_bas_Sprite.Cristal_Bleu_Bas_Sprite")
        (`SceneComponent.K2_SetRelativeLocation` _triangle2 (`|GetArrayItem` _m_trianglepositions 3) false false)))
    (`SceneComponent.SetVisibility` (`self.Triangle2`) true false)))

(fn `UserConstructionScript`
  (bind (_returnvalue_x _returnvalue_y _returnvalue_z) (`KismetMathLibrary.BreakVector` (`self.K2_GetActorLocation` (`self.M TowerSpot`))))
  (`SceneComponent.SetVisibility` (`self.Triangle1`) false false)
  (`SceneComponent.SetVisibility` (`self.Triangle2`) false false)
  (`/Engine/EditorBlueprintResources/StandardMacros.IsValid` (`self.M TowerSpot`)
    (:`Is Valid`
      (`self.K2_SetActorLocation` (`KismetMathLibrary.MakeVector` _returnvalue_x _returnvalue_y _returnvalue_z)))))