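; BP_HUB is a gameplay element actor that tracks its health and mirrors it on an attached health bar widget.
; SetHealth stores the new value, and LowerHealth subtracts an amount through it.
; Both then call UpdateWidgetHealth, which copies the value into the WBP_HUB_HealthBar obtained from the HealthBar component.
; The file applies no clamping and has no reaction to depleted health.
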(fn `GetHealthBar`
  (returns (Object :type "/Game/Blueprints/Widgets/HealthBars/WBP_HUB_HealthBar Object Reference"))
  (return (cast `/Game/Blueprints/Widgets/HealthBars/WBP_HUB_HealthBar` (`WidgetComponent.GetUserWidgetObject` (`self.HealthBar`)) :!pure true)))

(fn `LowerHealth`
  (params (Amount :type "Float (double-precision)"))
  (`self.SetHealth` (- (`self.M Health`) Amount))
  (`self.UpdateWidgetHealth`))

(fn `SetHealth`
  (params (NewHealth :type "Float (double-precision)"))
  (set `self.M Health` NewHealth)
  (`self.UpdateWidgetHealth`))

(fn `UpdateWidgetHealth`
  (bind _object (`self.GetHealthBar`))
  (set `/Game/Blueprints/Widgets/HealthBars/WBP_HUB_HealthBar.M Health` (`self.M Health`) _object))

(fn `UserConstructionScript`)