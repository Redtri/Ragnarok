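; BP_Goal is the level's goal actor: rats that reach it cost lives, and the player touching it after the assault is cleared returns to the HUB level.
; It creates the HUD and caches GM_PlayMode on BeginPlay.
; Rat overlaps trigger the rat's attack, subtract its type damage from lives, then update both HUD and game mode.
; An Appearing event spawns the hub-enabled effect, though its comment flags it as not working.
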(event `Appearing`
  ;[1 1 1] Appearing
  ;;[1 1 1] Not working
  (`ActorComponent.Activate` (`self.ParticleSystem`) false)
  (`GameplayStatics.SpawnEmitterAtLocation` "/Game/Particles/P_HubEnabled.P_HubEnabled" (`self.K2_GetActorLocation`)))

(event `self.ReceiveBeginPlay`
  ;[1 1 1] Init
  (`self.InitializeProperties`))

(event `self.ReceiveActorBeginOverlap`
  (params (OtherActor :type "Actor Object Reference"))
  (bind (_m_gamedata_lives _m_gamedata_score _m_gamedata_nbwaves) (break `/Game/Blueprints/Structs/STRUCT_GameData` (`self.M GameData`)))
  ;[1 1 1] Map Changing
  (cast `/Game/Blueprints/Players/BP_Player` OtherActor
    (:`then`
      (if (`/Game/Blueprints/Gamemodes/GM_PlayMode.M AssaultCleared` (`self.M GameModeRef`))
        (`self.LoadHUB`)))
    (:`CastFailed`
      ;[1 1 1] Receive rat damage
      (bind _asbp_base_rat (cast `/Game/Blueprints/Actors/Enemy/BP_BaseRat` OtherActor))
      (`/Game/Blueprints/Actors/Enemy/BP_BaseRat.Attack` _asbp_base_rat)
      (bind (_m_rattype_type _m_rattype_iscc _m_rattype_element _m_rattype_hp _m_rattype_speed _m_rattype_damage) (break `/Game/Blueprints/Structs/STRUCT_Rat` (`/Game/Blueprints/Actors/Enemy/BP_BaseRat.M RatType` _asbp_base_rat)))
      (bind _output_get (set `self.M GameData` (make `/Game/Blueprints/Structs/STRUCT_GameData` (- _m_gamedata_lives (`KismetMathLibrary.FTrunc` _m_rattype_damage)) _m_gamedata_score _m_gamedata_nbwaves)))
      (`self.RefreshWidgetInfos` _output_get)
      ;;[1 1 1] Refreshes GameMode data
      (`/Game/Blueprints/Gamemodes/GM_PlayMode.SetGameData` (`self.M GameModeRef`) (`self.M GameData`)))))

(event `LoadHUB`
  ;[1 1 1] Map Changing
  (bind _returnvalue (`|CreateWidget` "/Game/Blueprints/Widgets/HUB/WBP_LoadingScreen.WBP_LoadingScreen_C" (`GameplayStatics.GetPlayerController` 0)))
  (`UserWidget.AddToViewport` _returnvalue 0)
  (`GameplayStatics.OpenLevel` "HUB"))

(fn `GetDataFromGM`
  (returns (GameData :type "/Game/Blueprints/Structs/STRUCT_GameData Structure"))
  (return (`/Game/Blueprints/Gamemodes/GM_PlayMode.M GameData` (`self.M GameModeRef`))))

(fn `InitializeProperties`
  ;[1 1 1] Widget
  (bind _returnvalue (`|CreateWidget` "/Game/Blueprints/Widgets/HUB/WBP_HUD.WBP_HUD_C" (`GameplayStatics.GetPlayerController` 0)))
  (`UserWidget.AddToViewport` _returnvalue 0)
  (set `self.M WBP_HUB` _returnvalue)
  ;[1 1 1] GameMode
  (set `self.M GameModeRef` (cast `/Game/Blueprints/Gamemodes/GM_PlayMode` (`GameplayStatics.GetGameMode`) :!pure true)))

(fn `RefreshWidgetInfos`
  (params (Data :type "/Game/Blueprints/Structs/STRUCT_GameData Structure"))
  (bind _m_wbp_hub (`self.M WBP_HUB`))
  (`/Engine/EditorBlueprintResources/StandardMacros.IsValid` _m_wbp_hub
    (:`Is Valid`
      (`/Game/Blueprints/Widgets/HUB/WBP_HUD.RefreshInfos` _m_wbp_hub Data_Lives_6_7C54D35B4577DAD43C2B1B92DEE48D1A Data_Score_7_17FCA8A84EAD3FB8D64DDB9533DC9E7D Data_NbWaves_8_34A6FCF946A9AE92589234ACAC282B57))))

(fn `SetGameData`
  (params (GameData :type "/Game/Blueprints/Structs/STRUCT_GameData Structure"))
  (bind _output_get (set `self.M GameData` GameData))
  ;[1 1 1] Refreshes widget infos
  (`self.RefreshWidgetInfos` _output_get))

(fn `UserConstructionScript`)