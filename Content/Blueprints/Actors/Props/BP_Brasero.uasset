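; BP_Brasero is a brazier prop whose mesh follows an elemental influence skin.
; The UpdateSkin event swaps the static mesh to an earth variant for Earth and uses the normal brazier mesh for None, Fire, Wind and Water.
; The construction script runs the parent's script, then applies a random uniform scale and random yaw so placed copies vary.
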(event `self.UpdateSkin`
  (params (Influence :type "/Game/Blueprints/Enums/ENUM_Elem Enum" :default "NewEnumerator0"))
  (bind _mesh (`self.Mesh`))
  (switch `/Game/Blueprints/Enums/ENUM_Elem` Influence
    (:`NewEnumerator0`
      (`StaticMeshComponent.SetStaticMesh` _mesh "/Game/Meshes/Props/Brasero_normal.Brasero_normal" :!label _label))
    (:`NewEnumerator1`
      (goto _label))
    (:`NewEnumerator2`
      (goto _label))
    (:`NewEnumerator3`
      (`StaticMeshComponent.SetStaticMesh` _mesh "/Game/Meshes/Props/Brasero_terre_Brasero_terre.Brasero_terre_Brasero_terre"))
    (:`NewEnumerator4`
      (goto _label))))

(fn `UserConstructionScript`
  (`parent.UserConstructionScript`)
  (`self.SetActorScale3D` (`KismetMathLibrary.Conv_DoubleToVector` (`KismetMathLibrary.RandomFloatInRange` 1.0 1.5)))
  (`self.K2_SetActorRotation` (`KismetMathLibrary.MakeRotator` 0.0 0.0 (`KismetMathLibrary.RandomFloatInRange` 1.0 360.0))))