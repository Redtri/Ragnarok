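; Fountain prop that changes its static mesh according to an elemental influence.
; UpdateSkin gives None, Fire and Wind the normal fountain mesh, while Earth and Water both use the earth variant.
; The construction script runs the parent's logic, then applies a random uniform scale-down and a random yaw so placed fountains vary.
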(event `self.UpdateSkin`
  (params (Influence :type "/Game/Blueprints/Enums/ENUM_Elem Enum" :default "NewEnumerator0"))
  (bind _mesh (`self.Mesh`))
  (switch `/Game/Blueprints/Enums/ENUM_Elem` Influence
    (:`NewEnumerator0`
      (`StaticMeshComponent.SetStaticMesh` _mesh "/Game/Meshes/Props/fontaine_normal_fontaine_normal.fontaine_normal_fontaine_normal" :!label _label))
    (:`NewEnumerator1`
      (goto _label))
    (:`NewEnumerator2`
      (goto _label))
    (:`NewEnumerator3`
      (`StaticMeshComponent.SetStaticMesh` _mesh "/Game/Meshes/Props/fontaine_terre_fontaine_terre.fontaine_terre_fontaine_terre"))
    (:`NewEnumerator4`
      (`StaticMeshComponent.SetStaticMesh` _mesh "/Game/Meshes/Props/fontaine_terre_fontaine_terre.fontaine_terre_fontaine_terre"))))

(fn `UserConstructionScript`
  (`parent.UserConstructionScript`)
  (`self.SetActorScale3D` (`KismetMathLibrary.Conv_DoubleToVector` (`KismetMathLibrary.RandomFloatInRange` 0.5 0.7)))
  (`self.K2_SetActorRotation` (`KismetMathLibrary.MakeRotator` 0.0 0.0 (`KismetMathLibrary.RandomFloatInRange` 1.0 360.0))))