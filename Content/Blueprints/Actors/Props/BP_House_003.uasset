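; House prop variant whose static mesh changes to match an elemental influence.
; UpdateSkin switches on the influence: None and Fire share the normal house, while Wind, Earth and Water each get their own mesh.
; Earth and Water borrow 002-series meshes and add a relative rotation, which accumulates on repeated calls.
; The construction script runs the parent's setup, then uniformly scales the mesh down.
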(event `self.UpdateSkin`
  (params (Influence :type "/Game/Blueprints/Enums/ENUM_Elem Enum" :default "NewEnumerator0"))
  (bind _mesh (`self.Mesh`))
  (switch `/Game/Blueprints/Enums/ENUM_Elem` Influence
    (:`NewEnumerator0`
      (`StaticMeshComponent.SetStaticMesh` _mesh "/Game/Meshes/Houses/maison_normal003.maison_normal003" :!label _label))
    (:`NewEnumerator1`
      (goto _label))
    (:`NewEnumerator2`
      (`StaticMeshComponent.SetStaticMesh` _mesh "/Game/Meshes/Houses/maison_air003.maison_air003"))
    (:`NewEnumerator3`
      (`StaticMeshComponent.SetStaticMesh` _mesh "/Game/Meshes/Houses/maison_terre002.maison_terre002")
      (`SceneComponent.K2_AddRelativeRotation` _mesh (struct :`Yaw` 90.0) false false))
    (:`NewEnumerator4`
      (`StaticMeshComponent.SetStaticMesh` _mesh "/Game/Meshes/Houses/maison_eau002.maison_eau002")
      (`SceneComponent.K2_AddRelativeRotation` _mesh (struct :`Yaw` 180.0) false false))))

(fn `UserConstructionScript`
  (`parent.UserConstructionScript`)
  (`SceneComponent.SetRelativeScale3D` (`self.Mesh`) (0.4 0.4 0.4)))