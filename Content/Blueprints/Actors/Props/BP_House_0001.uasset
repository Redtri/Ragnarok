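; House prop actor that changes its appearance to match an elemental influence: none, fire, wind, earth or water.
; The UpdateSkin event swaps the static mesh for each influence and, for all but Fire, applies a mesh-specific yaw offset.
; The offset is added to the current rotation, so repeated updates accumulate.
; The construction script runs the parent's logic, then scales the mesh down uniformly.
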(event `self.UpdateSkin`
  (params (Influence :type "/Game/Blueprints/Enums/ENUM_Elem Enum" :default "NewEnumerator0"))
  (bind _mesh (`self.Mesh`))
  (switch `/Game/Blueprints/Enums/ENUM_Elem` Influence
    (:`NewEnumerator0`
      (`StaticMeshComponent.SetStaticMesh` _mesh "/Game/Meshes/Houses/maison_normal001.maison_normal001")
      (`SceneComponent.K2_AddRelativeRotation` _mesh (struct :`Yaw` -90.0) false false))
    (:`NewEnumerator1`
      (`StaticMeshComponent.SetStaticMesh` _mesh "/Game/Meshes/Houses/maison_feu003.maison_feu003"))
    (:`NewEnumerator2`
      (`StaticMeshComponent.SetStaticMesh` _mesh "/Game/Meshes/Houses/maison_air001.maison_air001")
      (`SceneComponent.K2_AddRelativeRotation` _mesh (struct :`Yaw` -90.0) false false))
    (:`NewEnumerator3`
      (`StaticMeshComponent.SetStaticMesh` _mesh "/Game/Meshes/Houses/maison_terre003.maison_terre003")
      (`SceneComponent.K2_AddRelativeRotation` _mesh (struct :`Yaw` 180.0) false false))
    (:`NewEnumerator4`
      (`StaticMeshComponent.SetStaticMesh` _mesh "/Game/Meshes/Houses/maison_eau004.maison_eau004")
      (`SceneComponent.K2_AddRelativeRotation` _mesh (struct :`Yaw` 90.0) false false))))

(fn `UserConstructionScript`
  (`parent.UserConstructionScript`)
  (`SceneComponent.SetRelativeScale3D` (`self.Mesh`) (0.4 0.4 0.4)))