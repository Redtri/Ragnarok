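; House prop variant that changes its appearance to match an elemental influence: None, Fire, Wind, Earth or Water.
; UpdateSkin swaps the static mesh per influence and adds a yaw offset for Fire, Earth and Water, which accumulates on repeated calls.
; Earth uses a water-named house mesh (Maison_eau001) and Water a tree mesh (Arbre_eau).
; The construction script runs the parent's, then uniformly shrinks the mesh.
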(event `self.UpdateSkin`
  (params (Influence :type "/Game/Blueprints/Enums/ENUM_Elem Enum" :default "NewEnumerator0"))
  (bind _mesh (`self.Mesh`))
  (switch `/Game/Blueprints/Enums/ENUM_Elem` Influence
    (:`NewEnumerator0`
      (`StaticMeshComponent.SetStaticMesh` _mesh "/Game/Meshes/Houses/maison_normal004.maison_normal004"))
    (:`NewEnumerator1`
      (`StaticMeshComponent.SetStaticMesh` _mesh "/Game/Meshes/Houses/maison_feu001.maison_feu001")
      (`SceneComponent.K2_AddRelativeRotation` _mesh (struct :`Yaw` 90.0) false false))
    (:`NewEnumerator2`
      (`StaticMeshComponent.SetStaticMesh` _mesh "/Game/Meshes/Houses/maison_air004.maison_air004"))
    (:`NewEnumerator3`
      (`StaticMeshComponent.SetStaticMesh` _mesh "/Game/Meshes/Houses/maison_eau001.maison_eau001")
      (`SceneComponent.K2_AddRelativeRotation` _mesh (struct :`Yaw` 180.0) false false))
    (:`NewEnumerator4`
      (`StaticMeshComponent.SetStaticMesh` _mesh "/Game/Meshes/Props/arbre_eau.arbre_eau")
      (`SceneComponent.K2_AddRelativeRotation` _mesh (struct :`Yaw` -90.0) false false))))

(fn `UserConstructionScript`
  (`parent.UserConstructionScript`)
  (`SceneComponent.SetRelativeScale3D` (`self.Mesh`) (0.4 0.4 0.4)))