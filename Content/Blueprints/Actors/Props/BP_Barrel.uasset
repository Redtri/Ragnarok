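; BP_Barrel is a barrel prop whose appearance changes with an elemental Influence.
; The UpdateSkin event swaps the static mesh, with dedicated Wind and Water models and the normal barrel for None, Fire and Earth.
; The construction script runs the parent's version, then randomizes uniform scale and yaw so placed barrels vary.
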(event `self.UpdateSkin`
  (params (Influence :type "/Game/Blueprints/Enums/ENUM_Elem Enum" :default "NewEnumerator0"))
  (bind _mesh (`self.Mesh`))
  (switch `/Game/Blueprints/Enums/ENUM_Elem` Influence
    (:`NewEnumerator0`
      (`StaticMeshComponent.SetStaticMesh` _mesh "/Game/Meshes/Props/Tonneau_normal_Tonneau_normal.Tonneau_normal_Tonneau_normal" :!label _label))
    (:`NewEnumerator1`
      (goto _label))
    (:`NewEnumerator2`
      (`StaticMeshComponent.SetStaticMesh` _mesh "/Game/Meshes/Props/Tonneau_air.Tonneau_air"))
    (:`NewEnumerator3`
      (goto _label))
    (:`NewEnumerator4`
      (`StaticMeshComponent.SetStaticMesh` _mesh "/Game/Meshes/Props/Tonneau_eau.Tonneau_eau"))))

(fn `UserConstructionScript`
  (`parent.UserConstructionScript`)
  (`self.SetActorScale3D` (`KismetMathLibrary.Conv_DoubleToVector` (`KismetMathLibrary.RandomFloatInRange` 1.0 2.0)))
  (`self.K2_SetActorRotation` (`KismetMathLibrary.MakeRotator` 0.0 0.0 (`KismetMathLibrary.RandomFloatInRange` 1.0 360.0))))