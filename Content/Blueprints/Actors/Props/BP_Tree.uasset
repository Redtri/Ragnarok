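; BP_Tree is a tree prop whose look follows an elemental influence.
; Its UpdateSkin event swaps the static mesh between a normal tree and fire, wind, earth and water variants.
; The construction script runs the parent's script, then gives the actor a random uniform scale and random yaw for visual variety.
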(event `self.UpdateSkin`
  (params (Influence :type "/Game/Blueprints/Enums/ENUM_Elem Enum" :default "NewEnumerator0"))
  (bind _mesh (`self.Mesh`))
  (switch `/Game/Blueprints/Enums/ENUM_Elem` Influence
    (:`NewEnumerator0`
      (`StaticMeshComponent.SetStaticMesh` _mesh "/Game/Meshes/Props/arbre_normal.arbre_normal"))
    (:`NewEnumerator1`
      (`StaticMeshComponent.SetStaticMesh` _mesh "/Game/Meshes/Props/arbre_feu.arbre_feu"))
    (:`NewEnumerator2`
      (`StaticMeshComponent.SetStaticMesh` _mesh "/Game/Meshes/Props/arbre_air.arbre_air"))
    (:`NewEnumerator3`
      (`StaticMeshComponent.SetStaticMesh` _mesh "/Game/Meshes/Props/arbre_terre.arbre_terre"))
    (:`NewEnumerator4`
      (`StaticMeshComponent.SetStaticMesh` _mesh "/Game/Meshes/Props/arbre_eau.arbre_eau"))))

(fn `UserConstructionScript`
  (`parent.UserConstructionScript`)
  (`self.SetActorScale3D` (`KismetMathLibrary.Conv_DoubleToVector` (`KismetMathLibrary.RandomFloatInRange` 10.0 20.0)))
  (`self.K2_SetActorRotation` (`KismetMathLibrary.MakeRotator` 0.0 0.0 (`KismetMathLibrary.RandomFloatInRange` 1.0 360.0))))