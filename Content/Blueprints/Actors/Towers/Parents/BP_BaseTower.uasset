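; Base actor for the rat-shooting elemental towers, configured on Init from game-mode data with per-type mesh, sounds, particles and targetable rat types.
; Tick handles cooldown, fills targets from all eligible rats up to a cap, and faces the first.
; Shots apply direct, splash and slow effects or spawn Ice spears, feeding the DPS meter.
; Each shot wears down the tower's lifetime until it sinks and frees its slot.
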(event `Init`
  (params (`Tower type` :type "/Game/Blueprints/Enums/ENUM_TowerType Enum" :default "NewEnumerator0") (TowerSpot :type "/Game/Blueprints/Actors/GameplayElement/BP_TowerSpawnPoint Object Reference"))
  (bind _value (`BlueprintMapLibrary.Map_Find` (`self.GetTowerSTDs`) `Tower type`))
  ;[1 1 1] Tower
  ;;[1 1 1] CONSTRUCTOR : Initializations : Tower type, shootable rats, sounds, particles
  (`self.InitializeProperties` _value TowerSpot)
  (`self.Spawning`)
  (bind (_direction _fallingcurve _scalingcurve _scalingmud) (`Timeline|SpawningTimeline`)
    (:`Update`
      (`self.K2_SetActorLocation` self (+ _fallingcurve (`self.M StartPos`)) false false)
      (`SceneComponent.SetWorldScale3D` (`self.Mesh`) (select `bool` (`|EnumEquality` (`.Type_8_5388C449488C3816862852B3DF0FDE77` (break `/Game/Blueprints/Structs/STRUCT_Tower` _value)) "NewEnumerator5") :`false` _scalingcurve :`true` _scalingmud)))
    (:`Finished`
      (`ActorComponent.Deactivate` (`self.Particles_Spawn`)))))

(event `CheckNewRat`
  (params (RatRef :type "/Game/Blueprints/Actors/Enemy/BP_BaseRat Object Reference"))
  (bind (_m_towertype_type _m_towertype_elem1 _m_towertype_elem2 _m_towertype_range _m_towertype_iscone _m_towertype_nbmaxtargets) (break `/Game/Blueprints/Structs/STRUCT_Tower` (`self.M TowerType`)))
  ;[1 1 1] Tower
  ;;[1 1 1 1 50] Handles focused rats
  (bind _return (`self.IsTypeOfRatShootable` (`/Game/Blueprints/Actors/Enemy/BP_BaseRat.M RatType` RatRef)))
  (if _return
    (if (< (`KismetArrayLibrary.Array_Length` (`self.M AimableRats`)) _m_towertype_nbmaxtargets)
      (`KismetArrayLibrary.Array_AddUnique` (`self.M AimableRats`) RatRef))))

(event `self.ReceiveTick`
  (params (DeltaSeconds :type "Float (single-precision)"))
  (bind _m_aimablerats (`self.M AimableRats`))
  (bind (_returnvalue_x _returnvalue_y _returnvalue_z) (`KismetMathLibrary.BreakVector` (`SceneComponent.K2_GetComponentLocation` (`self.DefaultSceneRoot`))))
  (bind _output (`|GetArrayItem` _m_aimablerats))
  (bind (_returnvalue_x_2 _returnvalue_y_2) (`KismetMathLibrary.BreakVector` (`SceneComponent.K2_GetComponentLocation` (`/Game/Blueprints/Actors/Enemy/BP_BaseRat.Capsule` _output))))
  ;[1 1 1] Tower
  ;;[1 1 1] Checking shot
  (`|ExecutionSequence`
    (:`then_0`
      (if (`self.M Dying`)
        _
        (elif (`self.M Reloading`)
          (bind _output_get (set `self.M CoolDown` (- (`self.M CoolDown`) DeltaSeconds)))
          (if (<= _output_get 0.0)
            (set `self.M Reloading` false)
            (`self.AcquireTargets` :!label _label))
          (else
            (goto _label)))))
    (:`then_1`
      (`KismetSystemLibrary.Delay` 0.2)
      (if (> (`KismetArrayLibrary.Array_Length` _m_aimablerats) 0)
        (`/Engine/EditorBlueprintResources/StandardMacros.IsValid` _output
          (:`Is Valid`
            (bind _output_get_2 (set `self.M Aiming` (`KismetMathLibrary.FindLookAtRotation` (`KismetMathLibrary.MakeVector` _returnvalue_x _returnvalue_y _returnvalue_z) (`KismetMathLibrary.MakeVector` _returnvalue_x_2 _returnvalue_y_2 _returnvalue_z))))
            (`self.K2_SetActorRotation` _output_get_2)))))))

(event `AcquireTargets`
  ;[1 1 1] Tower
  (bind _outactors (`GameplayStatics.GetAllActorsOfClass` "/Game/Blueprints/Actors/Enemy/BP_BaseRat.BP_BaseRat_C"))
  (for _array_element _outactors
    (`self.CheckNewRat` _array_element))
  (if (> (`KismetArrayLibrary.Array_Length` (`self.M AimableRats`)) 0)
    (`self.Shoot`)
    (else
      (`ActorComponent.Deactivate` (`self.Particles_Shot`)))))

(event `RemoveRat`
  (params (`Rat ref` :type "/Game/Blueprints/Actors/Enemy/BP_BaseRat Object Reference"))
  ;[1 1 1] Tower
  ;;[1 1 1 1 50] Handles focused rats
  (`KismetArrayLibrary.Array_RemoveItem` (`self.M AimableRats`) `Rat ref`))

(event `Shoot`
  (bind _healthbar (`self.GetHealthBar`))
  (bind _channel_shot (`self.Channel_Shot`))
  (bind (_m_towertype_type _m_towertype_elem1 _m_towertype_elem2 _m_towertype_range _m_towertype_iscone _m_towertype_nbmaxtargets _m_towertype_maxdamages _m_towertype_cooldown _m_towertype_damage _m_towertype_splashrange _m_towertype_splashdamage _m_towertype_slowforce _m_towertype_slowduration) (break `/Game/Blueprints/Structs/STRUCT_Tower` (`self.M TowerType`)))
  (bind _returnvalue (`KismetMathLibrary.FTrunc` _m_towertype_damage))
  (bind _returnvalue_2 (+ (`self.M CurrentPower`) _returnvalue))
  ;[1 1 1] Tower
  ;;[0 0 0] Shooting
  (`|ExecutionSequence`
    (:`then_0`
      ;;;[1 1 1] Polish effects
      (`ActorComponent.Activate` (`self.Particles_Shot`) true)
      (if (not (`AudioComponent.IsPlaying` _channel_shot))
        (`AudioComponent.SetSound` _channel_shot (`self.GetRandomSound` (`self.M ShotSounds`)))
        (`AudioComponent.Play` _channel_shot 0.0))
      ;;;[1 1 1] State values
      (set `self.M CoolDown` _m_towertype_cooldown)
      (set `self.M Reloading` true))
    (:`then_1`
      (for _array_element (`self.M AimableRats`)
        (`/Engine/EditorBlueprintResources/StandardMacros.IsValid` _array_element
          (:`Is Valid`
            (`ParticleSystemComponent.SetActorParameter` (`self.Particles_Shot`) "BeamTarget" _array_element)
            ;;;[1 1 1] Ice shot
            (if (`|EnumEquality` _m_towertype_type "NewEnumerator3")
              (bind _returnvalue_3 (`|SpawnActorFromClass` "/Game/Particles/BP_IceSpear.BP_IceSpear_C" (`self.GetTransform`) "Undefined" "OverrideRootScale" null null))
              (`/Game/Particles/BP_IceSpear.GoTo` _returnvalue_3 _array_element _m_towertype_damage _m_towertype_slowforce _m_towertype_slowduration)
              (`/Game/Particles/BP_IceSpear.SetTowerShooter` _returnvalue_3 (`self.M TowerType`))
              (else
                (if (> _m_towertype_splashrange 0.0)
                  ;;;[1 1 1] Splash shot
                  (bind _outactors (`GameplayStatics.GetAllActorsOfClass` "/Game/Blueprints/Actors/Enemy/BP_BaseRat.BP_BaseRat_C"))
                  (for _array_element_2 _outactors
                    (`/Engine/EditorBlueprintResources/StandardMacros.IsValid` _array_element_2
                      (:`Is Valid`
                        (if (!= _array_element_2 _array_element)
                          (if (<= (`KismetMathLibrary.VSize` (- (`self.K2_GetActorLocation` _array_element) (`self.K2_GetActorLocation` _array_element_2))) _m_towertype_splashrange)
                            (bind _stillalive (`/Game/Blueprints/Actors/Enemy/BP_BaseRat.ReceiveDamages` _array_element_2 _m_towertype_splashdamage _m_towertype_slowforce _m_towertype_slowduration))
                            (if (not _stillalive)
                              (`/Game/Blueprints/Actors/Enemy/BP_BaseRat.Death` _array_element_2)
                              (`self.RemoveRat` _array_element_2))
                            ;;[1 1 1] Refreshing DPS Meter values
                            (`/Game/Blueprints/Gamemodes/GM_PlayMode.AddDamagesFromTower` (`self.M GameModeRef`) (`self.M TowerType`) _m_towertype_splashdamage)))))))
                ;;;[1 1 1] Classic shot
                (bind _stillalive_2 (`/Game/Blueprints/Actors/Enemy/BP_BaseRat.ReceiveDamages` _array_element _m_towertype_damage _m_towertype_slowforce _m_towertype_slowduration))
                (if (not _stillalive_2)
                  (`/Game/Blueprints/Actors/Enemy/BP_BaseRat.Death` _array_element)
                  (`self.RemoveRat` _array_element))
                (`/Game/Blueprints/Gamemodes/GM_PlayMode.AddDamagesFromTower` (`self.M GameModeRef`) (`self.M TowerType`) _m_towertype_damage))))))
      ;;;[1 1 1] Lifetime
      (`/Game/Blueprints/Widgets/HealthBars/WBP_TowerHealthBar.RefreshHpLoss` _healthbar _returnvalue)
      (set `/Game/Blueprints/Widgets/HealthBars/WBP_TowerHealthBar.M Health` (- 1.0 (/ (`KismetMathLibrary.Conv_IntToDouble` _returnvalue_2) (`KismetMathLibrary.Conv_IntToDouble` _m_towertype_maxdamages))) _healthbar)
      (bind _output_get (set `self.M CurrentPower` _returnvalue_2))
      ;;;[1 0 0.001108] Add destroy animation here
      (if (>= _output_get _m_towertype_maxdamages)
        (`ActorComponent.Activate` (`self.Particles_Spawn`) true)
        ;;;[1 1 1] Tower death
        (set `self.M Dying` true)
        (bind (_direction _sinkmult) (`Timeline|Sinking` :!via `PlayFromStart`)
          (:`Update`
            (`self.K2_AddActorWorldOffset` self (`KismetMathLibrary.MakeVector` 0.0 0.0 (* _sinkmult -1.0)) false false))
          (:`Finished`
            (set `/Game/Blueprints/Actors/GameplayElement/BP_TowerSpawnPoint.M IsFreeSlot` true (`self.M TowerSpot`))
            (`self.K2_DestroyActor`)))))))

(fn `CanShoot`
  (params (Rat :type "/Game/Blueprints/Structs/STRUCT_Rat Structure"))
  (returns (Return :type Boolean))
  ;[1 0 0.001338 1 50] WATCH OUT
  (for _array_element (`self.M ShootableRats`)
    (if (`|EnumEquality` (break `/Game/Blueprints/Structs/STRUCT_Rat` _array_element) Rat_Type_31_D1C7238147C1A92B1BFC6CB0EE96F39A)
      (return true)))
  (return false))

(fn `GetShootableRats`
  (params (`Tower type` :type "/Game/Blueprints/Enums/ENUM_TowerType Enum" :default "NewEnumerator0"))
  (returns (Return :type "Array of /Game/Blueprints/Structs/STRUCT_Rat Structure"))
  (locals (FillingShootables :type "Array of /Game/Blueprints/Structs/STRUCT_Rat Structure"))
  (bind _fillingshootables (`local.FillingShootables`))
  (bind _values (`BlueprintMapLibrary.Map_Values` (`self.GetRatSTDs`)))
  (for _array_element _values
    (bind (_type _iscc) (break `/Game/Blueprints/Structs/STRUCT_Rat` _array_element))
    (if (`|EnumEquality` _type "NewEnumerator0")
      (`KismetArrayLibrary.Array_Add` _fillingshootables _array_element :!label _label)
      (else
        (switch `/Game/Blueprints/Enums/ENUM_TowerType` `Tower type`
          (:`NewEnumerator0`
            (bind _returnvalue (`|EnumInequality` _type "NewEnumerator1"))
            (if _returnvalue :!label _label_2
              (if (`|EnumInequality` _type "NewEnumerator4") :!label _label_3
                (goto _label))))
          (:`NewEnumerator1`
            (goto _label_3))
          (:`NewEnumerator2`
            (bind _returnvalue_2 (not _iscc))
            (if _returnvalue_2
              (goto _label_3)))
          (:`NewEnumerator3`
            (goto _label_3))
          (:`NewEnumerator4`
            (if (and _returnvalue _returnvalue_2)
              (goto _label_3)))
          (:`NewEnumerator5`
            (goto _label_3))
          (:`NewEnumerator6`
            (goto _label_2))
          (:`NewEnumerator7`
            (goto _label_2))
          (:`NewEnumerator8`
            (goto _label_3))
          (:`NewEnumerator9`
            (goto _label_2))))))
  (return _fillingshootables))

(fn `InitializeProperties`
  (params (TowerType :type "/Game/Blueprints/Structs/STRUCT_Tower Structure") (TowerSpot :type "/Game/Blueprints/Actors/GameplayElement/BP_TowerSpawnPoint Object Reference"))
  (set `self.M StartPos` (`self.K2_GetActorLocation`))
  (bind _output_get (set `self.M TowerType` TowerType))
  ;[1 1 1] Shootable rats
  (bind _return (`self.GetShootableRats` (break `/Game/Blueprints/Structs/STRUCT_Tower` _output_get)))
  (set `self.M ShootableRats` _return)
  ;[1 1 1] Sounds
  (`self.SetProperSounds` (break `/Game/Blueprints/Structs/STRUCT_Tower` _output_get))
  ;[1 1 1] Particles
  (`ParticleSystemComponent.SetVectorParameter` (`self.Particles_Spawn`) "ParamTowerColor" (`KismetMathLibrary.Conv_LinearColorToVector` (select `/Game/Blueprints/Enums/ENUM_TowerType` (break `/Game/Blueprints/Structs/STRUCT_Tower` _output_get) :`NewEnumerator0` (struct :`R` 0.504167 :`G` 0.014261 :`A` 1.0) :`NewEnumerator1` (struct :`R` 0.094118 :`G` 0.701961 :`B` 0.666667 :`A` 1.0) :`NewEnumerator2` (struct :`R` 1.0 :`G` 1.0 :`B` 1.0 :`A` 1.0) :`NewEnumerator3` (struct :`G` 0.47451 :`B` 0.811765 :`A` 1.0) :`NewEnumerator4` (struct :`G` 0.063649 :`B` 0.936 :`A` 1.0) :`NewEnumerator5` (struct :`R` 0.920833 :`G` 0.160797 :`B` 0.043167 :`A` 1.0) :`NewEnumerator6` (struct :`R` 0.20242 :`G` 0.733333 :`B` 0.313478 :`A` 1.0) :`NewEnumerator7` (struct :`R` 0.592 :`G` 0.196544 :`A` 1.0) :`NewEnumerator8` (struct :`R` 0.4875 :`G` 0.410985 :`B` 0.063381 :`A` 1.0) :`NewEnumerator9` (struct :`R` 0.941667 :`G` 0.176562 :`B` 0.530249 :`A` 1.0) :!type "LinearColor Structure")))
  (`self.SetProperParticles` (break `/Game/Blueprints/Structs/STRUCT_Tower` _output_get))
  ;[1 1 1] Mesh
  (`self.SetProperMesh` (break `/Game/Blueprints/Structs/STRUCT_Tower` _output_get))
  ;[1 1 1] References
  (set `self.M GameModeRef` (cast `/Game/Blueprints/Gamemodes/GM_PlayMode` (`GameplayStatics.GetGameMode`) :!pure true))
  (bind _returnvalue (`|CreateWidget` "/Game/Blueprints/Widgets/HealthBars/WBP_TowerHealthBar.WBP_TowerHealthBar_C"))
  (`WidgetComponent.SetWidget` (`self.HealthBar`) _returnvalue)
  (set `/Game/Blueprints/Widgets/HealthBars/WBP_TowerHealthBar.M Health` 100.0 (`self.GetHealthBar`))
  (bind _output_get_2 (set `self.M TowerSpot` TowerSpot))
  (`KismetSystemLibrary.PrintString` (`KismetStringLibrary.Concat_StrStr` "Add " (`KismetSystemLibrary.GetDisplayName` _output_get_2))))

(fn `IsTypeOfRatShootable`
  (params (Rat :type "/Game/Blueprints/Structs/STRUCT_Rat Structure"))
  (returns (Return :type Boolean))
  (for _array_element (`self.M ShootableRats`)
    (if (`self.RatStructEqual` _array_element Rat)
      (return true)))
  (return false))

(fn `SetProperMesh`
  (params (TowerType :type "/Game/Blueprints/Enums/ENUM_TowerType Enum" :default "NewEnumerator0"))
  (bind _mesh (`self.Mesh`))
  (switch `/Game/Blueprints/Enums/ENUM_TowerType` TowerType
    (:`NewEnumerator0`
      (`StaticMeshComponent.SetStaticMesh` _mesh "/Game/Meshes/Towers/Fire_tower.Fire_tower")
      (set `self.M Scale` 1.0 :!label _label))
    (:`NewEnumerator1`
      (`StaticMeshComponent.SetStaticMesh` _mesh "/Game/Meshes/Towers/Thunder_tower.Thunder_tower")
      (goto _label))
    (:`NewEnumerator2`
      (`StaticMeshComponent.SetStaticMesh` _mesh "/Game/Meshes/Towers/Air_tower.Air_tower")
      (`SceneComponent.K2_AddRelativeRotation` _mesh (struct :`Yaw` -90.0) false false :!label _label_2)
      (goto _label))
    (:`NewEnumerator3`
      (`StaticMeshComponent.SetStaticMesh` _mesh "/Game/Meshes/Towers/Ice_tower.Ice_tower")
      (goto _label))
    (:`NewEnumerator4`
      (`StaticMeshComponent.SetStaticMesh` _mesh "/Game/Meshes/Towers/Water_tower.Water_tower"))
    (:`NewEnumerator5`
      (`StaticMeshComponent.SetStaticMesh` _mesh "/Game/Meshes/Towers/Geyser_Tower.Geyser_Tower")
      (set `self.M Scale` 0.5))
    (:`NewEnumerator6`
      (`StaticMeshComponent.SetStaticMesh` _mesh "/Game/Meshes/Towers/Earth_tower.Earth_tower")
      (goto _label_2))
    (:`NewEnumerator7`
      (`StaticMeshComponent.SetStaticMesh` _mesh "/Game/Meshes/Towers/Volcano_tower.Volcano_tower")
      (goto _label))
    (:`NewEnumerator8`
      (`StaticMeshComponent.SetStaticMesh` _mesh "/Game/Meshes/Towers/Sand_tower.Sand_tower")
      (goto _label))
    (:`NewEnumerator9`
      (`StaticMeshComponent.SetStaticMesh` _mesh "/Game/Meshes/Towers/Laser_tower.Laser_tower")
      (goto _label))))

(fn `SetProperParticles`
  (params (TowerType :type "/Game/Blueprints/Enums/ENUM_TowerType Enum" :default "NewEnumerator0"))
  (bind _particles_shot (`self.Particles_Shot`))
  (bind _particles_shot_2 (`self.Particles_Shot`))
  (bind _particles_shot_3 (`self.Particles_Shot`))
  (switch `/Game/Blueprints/Enums/ENUM_TowerType` TowerType
    (:`NewEnumerator0`
      (`ParticleSystemComponent.SetTemplate` (`self.Particles_Shot`) "/Game/Particles/P_Fire.P_Fire")
      ;[1 1 1] Scaling it up
      (`SceneComponent.SetWorldScale3D` (`self.Particles_Shot`) (3.0 3.0 3.0) :!label _label))
    (:`NewEnumerator1`
      (`ParticleSystemComponent.SetTemplate` (`self.Particles_Shot`) "/Game/Particles/P_Beam.P_Beam")
      (`ParticleSystemComponent.SetBeamSourcePoint` _particles_shot_2 0 (`self.K2_GetActorLocation`) 0)
      (`ParticleSystemComponent.SetActorParameter` _particles_shot_2 "BeamSource" self))
    (:`NewEnumerator2`
      (`ParticleSystemComponent.SetTemplate` (`self.Particles_Shot`) "/Game/Particles/P_Tornado.P_Tornado"))
    (:`NewEnumerator3`
      (`ParticleSystemComponent.SetTemplate` (`self.Particles_Shot`) "/Game/Particles/P_Snowflake.P_Snowflake"))
    (:`NewEnumerator4`
      (`ParticleSystemComponent.SetTemplate` (`self.Particles_Shot`) "/Game/Particles/P_WaterWater.P_WaterWater")
      (goto _label))
    (:`NewEnumerator5`
      (`ParticleSystemComponent.SetTemplate` _particles_shot_3 "/Game/Particles/P_GeyserSplash.P_GeyserSplash")
      (`SceneComponent.K2_AddRelativeLocation` _particles_shot_3 (0.0 0.0 80.0) false false))
    (:`NewEnumerator6`
      (`ParticleSystemComponent.SetTemplate` (`self.Particles_Shot`) "/Game/Particles/P_Earthquake.P_Earthquake"))
    (:`NewEnumerator7`
      (`ParticleSystemComponent.SetTemplate` (`self.Particles_Shot`) "/Game/Particles/P_Lava.P_Lava"))
    (:`NewEnumerator8`
      (`ParticleSystemComponent.SetTemplate` (`self.Particles_Shot`) "/Game/Particles/P_Sandstorm.P_Sandstorm"))
    (:`NewEnumerator9`
      (`ParticleSystemComponent.SetTemplate` _particles_shot "/Game/Particles/P_Beam1.P_Beam1")
      (`SceneComponent.K2_AddRelativeRotation` _particles_shot (struct :`Yaw` 90.0) false false)
      (`SceneComponent.K2_AddRelativeLocation` _particles_shot (300.0 0.0 0.0) false false))))

(fn `SetProperSounds`
  (params (TowerType :type "/Game/Blueprints/Enums/ENUM_TowerType Enum" :default "NewEnumerator0"))
  (bind _m_shotsounds (`self.M ShotSounds`))
  (bind _m_shotsounds_2 (`self.M ShotSounds`))
  (bind _m_shotsounds_3 (`self.M ShotSounds`))
  (bind _m_shotsounds_4 (`self.M ShotSounds`))
  (bind _m_shotsounds_5 (`self.M ShotSounds`))
  (switch `/Game/Blueprints/Enums/ENUM_TowerType` TowerType
    (:`NewEnumerator0`
      (`KismetArrayLibrary.Array_Add` (`self.M ShotSounds`) "/Game/Sounds/Tower_sounds/Tower-Fire-Attack-Loop.Tower-Fire-Attack-Loop")
      (`KismetArrayLibrary.Array_Add` (`self.M SpawnSounds`) "/Game/Sounds/Tower_sounds/Tower-Fire-Intro.Tower-Fire-Intro"))
    (:`NewEnumerator1`
      (`KismetArrayLibrary.Array_Add` _m_shotsounds "/Game/Sounds/Tower_sounds/Tower-Thunder-Attack-1.Tower-Thunder-Attack-1")
      (`KismetArrayLibrary.Array_Add` _m_shotsounds "/Game/Sounds/Tower_sounds/Tower-Thunder-Attack-2.Tower-Thunder-Attack-2")
      (`KismetArrayLibrary.Array_Add` (`self.M SpawnSounds`) "/Game/Sounds/Tower_sounds/Tower-Thunder-Intro.Tower-Thunder-Intro"))
    (:`NewEnumerator2`
      (`KismetArrayLibrary.Array_Add` _m_shotsounds_3 "/Game/Sounds/Tower_sounds/Tower-Wind-Attack-1.Tower-Wind-Attack-1")
      (`KismetArrayLibrary.Array_Add` _m_shotsounds_3 "/Game/Sounds/Tower_sounds/Tower-Wind-Attack-2.Tower-Wind-Attack-2")
      (`KismetArrayLibrary.Array_Add` _m_shotsounds_3 "/Game/Sounds/Tower_sounds/Tower-Wind-Attack-3.Tower-Wind-Attack-3")
      (`KismetArrayLibrary.Array_Add` (`self.M SpawnSounds`) "/Game/Sounds/Tower_sounds/Tower-Wind-Intro.Tower-Wind-Intro"))
    (:`NewEnumerator3`
      (`KismetArrayLibrary.Array_Add` (`self.M ShotSounds`) "/Game/Sounds/Tower_sounds/Tower-Ice-Attack-1.Tower-Ice-Attack-1")
      (`KismetArrayLibrary.Array_Add` (`self.M SpawnSounds`) "/Game/Sounds/Tower_sounds/Tower-Ice-Intro.Tower-Ice-Intro"))
    (:`NewEnumerator4`
      (`KismetArrayLibrary.Array_Add` (`self.M ShotSounds`) "/Game/Sounds/Tower_sounds/Tower-Water-Attack-Loop.Tower-Water-Attack-Loop")
      (`KismetArrayLibrary.Array_Add` (`self.M SpawnSounds`) "/Game/Sounds/Tower_sounds/Tower-Water-Intro.Tower-Water-Intro"))
    (:`NewEnumerator5`
      (`KismetArrayLibrary.Array_Add` (`self.M ShotSounds`) "/Game/Sounds/Tower_sounds/Tower-Mud-Attack-Launch.Tower-Mud-Attack-Launch")
      (`KismetArrayLibrary.Array_Add` (`self.M SpawnSounds`) "/Game/Sounds/Tower_sounds/Tower-Mud-Intro.Tower-Mud-Intro"))
    (:`NewEnumerator6`
      (`KismetArrayLibrary.Array_Add` (`self.M ShotSounds`) "/Game/Sounds/Tower_sounds/Tower-Earth-Attack-Loop.Tower-Earth-Attack-Loop")
      (`KismetArrayLibrary.Array_Add` (`self.M SpawnSounds`) "/Game/Sounds/Tower_sounds/Tower-Earth-Intro.Tower-Earth-Intro"))
    (:`NewEnumerator7`
      (`KismetArrayLibrary.Array_Add` _m_shotsounds_4 "/Game/Sounds/Tower_sounds/Tower-Lava-Attack-1.Tower-Lava-Attack-1")
      (`KismetArrayLibrary.Array_Add` _m_shotsounds_4 "/Game/Sounds/Tower_sounds/Tower-Lava-Attack-2.Tower-Lava-Attack-2")
      (`KismetArrayLibrary.Array_Add` (`self.M SpawnSounds`) "/Game/Sounds/Tower_sounds/Tower-Lava-Intro.Tower-Lava-Intro"))
    (:`NewEnumerator8`
      (`KismetArrayLibrary.Array_Add` _m_shotsounds_5 "/Game/Sounds/Tower_sounds/Tower-Sand-Attack-1.Tower-Sand-Attack-1")
      (`KismetArrayLibrary.Array_Add` _m_shotsounds_5 "/Game/Sounds/Tower_sounds/Tower-Sand-Attack-2.Tower-Sand-Attack-2")
      (`KismetArrayLibrary.Array_Add` _m_shotsounds_5 "/Game/Sounds/Tower_sounds/Tower-Sand-Attack-3.Tower-Sand-Attack-3")
      (`KismetArrayLibrary.Array_Add` _m_shotsounds_5 "/Game/Sounds/Tower_sounds/Tower-Sand-Attack-4.Tower-Sand-Attack-4")
      (`KismetArrayLibrary.Array_Add` (`self.M SpawnSounds`) "/Game/Sounds/Tower_sounds/Tower-Sand-Intro.Tower-Sand-Intro"))
    (:`NewEnumerator9`
      (`KismetArrayLibrary.Array_Add` _m_shotsounds_2 "/Game/Sounds/Tower_sounds/Tower-Laser-Attack-1.Tower-Laser-Attack-1")
      (`KismetArrayLibrary.Array_Add` _m_shotsounds_2 "/Game/Sounds/Tower_sounds/Tower-Laser-Attack-2.Tower-Laser-Attack-2")
      (`KismetArrayLibrary.Array_Add` _m_shotsounds_2 "/Game/Sounds/Tower_sounds/Tower-Laser-Attack-3.Tower-Laser-Attack-3")
      (`KismetArrayLibrary.Array_Add` (`self.M SpawnSounds`) "/Game/Sounds/Tower_sounds/Tower-Laser-Intro.Tower-Laser-Intro"))))

(fn `Spawning`
  (bind _channel_state (`self.Channel_State`))
  (`AudioComponent.SetSound` _channel_state (`self.GetRandomSound` (`self.M SpawnSounds`)))
  (`AudioComponent.Play` _channel_state 0.0)
  (`ActorComponent.Activate` (`self.Particles_Spawn`) false))

(fn `UserConstructionScript`)