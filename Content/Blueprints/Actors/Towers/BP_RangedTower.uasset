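; Ranged tower actor that detects rats within its range and fires at them, extending a parent tower class.
; On init it sizes the TriggerRange box from the tower type's range, offsetting and rotating it forward for cone types.
; Overlap events pass entering rats to CheckNewRat and remove shootable ones that leave.
; AcquireTargets rescans overlapping rats, then calls the parent's shoot if any are aimable or stops the shot particles.
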(event `self.Init`
  (params (`Tower type` :type "/Game/Blueprints/Enums/ENUM_TowerType Enum" :default "NewEnumerator0") (TowerSpot :type "/Game/Blueprints/Actors/GameplayElement/BP_TowerSpawnPoint Object Reference"))
  (bind (_m_towertype_type _m_towertype_elem1 _m_towertype_elem2 _m_towertype_range _m_towertype_iscone) (break `/Game/Blueprints/Structs/STRUCT_Tower` (`self.M TowerType`)))
  (bind _trigger_range (`self.Trigger_Range`))
  (bind _returnvalue (* _m_towertype_range 10.0))
  ;[1 1 1] CONSTRUCTOR : Range size
  (`parent.Init` `Tower type` TowerSpot)
  (if _m_towertype_iscone
    (`BoxComponent.SetBoxExtent` _trigger_range (`KismetMathLibrary.MakeVector` 64.0 _returnvalue 500.0) true)
    (`SceneComponent.K2_SetRelativeRotation` _trigger_range (`KismetMathLibrary.MakeRotator` 0.0 0.0 90.0) false false)
    (`SceneComponent.K2_SetRelativeLocation` _trigger_range (`KismetMathLibrary.MakeVector` _returnvalue) false false)
    (else
      (`BoxComponent.SetBoxExtent` (`self.Trigger_Range`) (`KismetMathLibrary.MakeVector` _returnvalue _returnvalue 500.0) true))))

(event `self.Trigger_Range.OnComponentBeginOverlap`
  (params (OverlappedComponent :type "PrimitiveComponent Object Reference") (OtherActor :type "Actor Object Reference") (OtherComp :type "PrimitiveComponent Object Reference") (OtherBodyIndex :type Integer) (bFromSweep :type Boolean) (SweepResult :type "HitResult Structure (by ref)"))
  ;[1 1 1] TARGETS : Adding and removing
  ;;[1 0 0.005438] CHECK NB MAX TARGET ?
  (bind _asbp_base_rat (cast `/Game/Blueprints/Actors/Enemy/BP_BaseRat` OtherActor))
  (`self.CheckNewRat` _asbp_base_rat))

(event `self.Trigger_Range.OnComponentEndOverlap`
  (params (OverlappedComponent :type "PrimitiveComponent Object Reference") (OtherActor :type "Actor Object Reference") (OtherComp :type "PrimitiveComponent Object Reference") (OtherBodyIndex :type Integer))
  ;[1 1 1] TARGETS : Adding and removing
  (bind _asbp_base_rat (cast `/Game/Blueprints/Actors/Enemy/BP_BaseRat` OtherActor))
  (bind _return (`self.IsTypeOfRatShootable` (`/Game/Blueprints/Actors/Enemy/BP_BaseRat.M RatType` _asbp_base_rat)))
  (if _return
    (`self.RemoveRat` _asbp_base_rat)))

(event `self.AcquireTargets`
  (for _array_element (`PrimitiveComponent.GetOverlappingActors` (`self.Trigger_Range`) "/Game/Blueprints/Actors/Enemy/BP_BaseRat.BP_BaseRat_C")
    (bind _asbp_base_rat (cast `/Game/Blueprints/Actors/Enemy/BP_BaseRat` _array_element))
    (`self.CheckNewRat` _asbp_base_rat))
  (if (> (`KismetArrayLibrary.Array_Length` (`self.M AimableRats`)) 0)
    (`parent.Shoot`)
    (else
      (`ActorComponent.Deactivate` (`self.Particles_Shot`)))))

(fn `UserConstructionScript`
  (`parent.UserConstructionScript`))