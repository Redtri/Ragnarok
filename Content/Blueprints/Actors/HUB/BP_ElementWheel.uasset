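; Element wheel actor for the HUB that spins to face the given elemental Influence (Fire, Wind, Earth or Water).
; TurnWheel plays all four element audio components and runs the Turning timeline, lerping the roll of Datas from 360 degrees to that element's angle.
; Past the timeline's midpoint, a one-shot MFading flag fades the element audio out.
; On finish, AudioEvent plays and the BITE effect, tinted white at construction, deactivates.
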(event `TurnWheel`
  (params (Influence :type "/Game/Blueprints/Enums/ENUM_Elem Enum" :default "NewEnumerator0"))
  (bind _audio_fire (`self.Audio_Fire`))
  (bind _turning (`self.Turning`))
  (bind _returnvalue (`TimelineComponent.GetPlaybackPosition` _turning))
  (`AudioComponent.Play` _audio_fire 0.0)
  (`AudioComponent.Play` (`self.Audio_Wind`) 0.0)
  (`AudioComponent.Play` (`self.Audio_Earth`) 0.0)
  (`AudioComponent.Play` (`self.Audio_Water`) 0.0)
  (bind (_direction _alpha) (`Timeline|Turning` :!via `PlayFromStart`)
    (:`Update`
      (`SceneComponent.K2_SetRelativeRotation` (`self.Datas`) (`KismetMathLibrary.MakeRotator` (`KismetMathLibrary.Lerp` 360.0 (select `/Game/Blueprints/Enums/ENUM_Elem` Influence :`NewEnumerator1` -90.0 :`NewEnumerator3` 180.0 :`NewEnumerator4` 90.0 :!type "Float (single-precision)") _alpha) 90.0) false false)
      (if (> _returnvalue 0.0)
        (if (and (not (`self.M Fading`)) (<= (/ (`TimelineComponent.GetTimelineLength` _turning) _returnvalue) 2.0))
          (set `self.M Fading` true)
          (`AudioComponent.FadeOut` _audio_fire 6.0 0.0)
          (`AudioComponent.FadeOut` (`self.Audio_Wind`) 6.0 0.0)
          (`AudioComponent.FadeOut` (`self.Audio_Earth`) 6.0 0.0)
          (`AudioComponent.FadeOut` (`self.Audio_Water`) 6.0 0.0))))
    (:`Finished`
      (`AudioComponent.Play` (`self.Audio_Event`) 0.0)
      (`ActorComponent.Deactivate` (`self.BITE`)))))

(fn `UserConstructionScript`
  (`ParticleSystemComponent.SetVectorParameter` (`self.BITE`) "ParamTowerColor" (`KismetMathLibrary.Conv_LinearColorToVector` (struct :`R` 1.0 :`G` 1.0 :`B` 1.0 :`A` 1.0))))