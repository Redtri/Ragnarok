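; Base enemy rat actor that advances on BP_Goal and can attack, take damage, be slowed, and die.
; Init pulls the type's stats from GM_PlayMode, then fills flipbook and sound lists per rat type and upgrade state.
; Ground rats path with AIMoveTo while Tick picks directional flipbooks from velocity; flying rats are raised and steered by manual offsets.
; Attack and Death report removal to the play mode before destroying the actor.
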(event `Death`
  ;[1 0.4233 0.09937] Death
  (`KismetSystemLibrary.Delay` 0.5)
  (`/Game/Blueprints/Gamemodes/GM_PlayMode.RemoveRat` (`self.GetPlayMode`) self true)
  (`self.K2_DestroyActor`))

(event `Init`
  (params (RatType :type "/Game/Blueprints/Enums/ENUM_RatType Enum" :default "NewEnumerator0") (IsUpgraded :type Boolean))
  ;[0 0.05339 1] CONSTRUCTOR
  (`self.InitializeProperties` (`BlueprintMapLibrary.Map_Find` (`self.GetRatsSTDs`) RatType) IsUpgraded))

(event `Movement`
  ;[1 1 1] Movement
  (if (not (or (`self.M IsDying`) (`self.M IsAttacking`)))
    (`|AIMoveTo` self (0.0 0.0 0.0) (`self.Goal`))))

(event `Attack`
  (bind _channel_event_bis (`self.Channel_Event_bis`))
  ;[1 1 1] Attack
  (set `self.M IsAttacking` true)
  (`AudioComponent.SetSound` _channel_event_bis (`self.RandomSoundFrom` (break `/Game/Blueprints/Structs/STRUCT_AudioContainer` (`BlueprintMapLibrary.Map_Find` (`self.M Sounds`) "NewEnumerator0"))))
  (`AudioComponent.Play` _channel_event_bis 0.0)
  (`PaperFlipbookComponent.SetFlipbook` (`self.PaperFlipbook`) (`|GetArrayItem` (`self.M Animations`) (`self.INDEX_Attack`)))
  (`/Game/Blueprints/Gamemodes/GM_PlayMode.RemoveRat` (`self.GetPlayMode`) self false)
  (`KismetSystemLibrary.Delay` 1.0)
  (`self.K2_DestroyActor`))

(event `self.ReceiveActorBeginOverlap`
  (params (OtherActor :type "Actor Object Reference"))
  ;[1 0 0.8488] STOP AT GOAL
  (if (== (`GameplayStatics.GetObjectClass` OtherActor) "/Game/Blueprints/Actors/GameplayElement/BP_Goal.BP_Goal_C")
    (`NavMovementComponent.StopActiveMovement` (`self.FloatingPawnMovement`))
    (set `self.isGoal` true)))

(event `self.ReceiveTick`
  (params (DeltaSeconds :type "Float (single-precision)"))
  (bind _m_animations (`self.M Animations`))
  (bind (_m_rattype_type _m_rattype_iscc _m_rattype_element _m_rattype_hp _m_rattype_speed) (break `/Game/Blueprints/Structs/STRUCT_Rat` (`self.M RatType`)))
  (bind _paperflipbook (`self.PaperFlipbook`))
  (bind _m_rattype_type_2 (break `/Game/Blueprints/Structs/STRUCT_Rat` (`self.M RatType`)))
  (bind _paperflipbook_2 (`self.PaperFlipbook`))
  (bind _x (.x (`MovementComponent.Velocity` (`self.FloatingPawnMovement`))))
  (bind _y (.y (`MovementComponent.Velocity` (`self.FloatingPawnMovement`))))
  (bind _returnvalue (> _y 0.0))
  (if (`self.M IsSlowed`)
    (bind _output_get (set `self.M SlowDuration` (- (`self.M SlowDuration`) DeltaSeconds)))
    (if (<= _output_get 0.0)
      (set `self.M IsSlowed` false)
      (set `FloatingPawnMovement.MaxSpeed` _m_rattype_speed (`self.FloatingPawnMovement`))))
  (if (or (`self.M IsAttacking`) (`self.M IsDying`))
    (`NavMovementComponent.StopActiveMovement` (`self.FloatingPawnMovement`))
    (elif (`|EnumEquality` _m_rattype_type_2 "NewEnumerator1")
      (if _returnvalue
        ;[1 0.9502 0.04714] RIGHT
        (`SceneComponent.K2_SetWorldRotation` _paperflipbook_2 (struct :`Yaw` -90.0 :`Roll` 90.0) false false)
        (else
          ;[0.01382 1 0.1518] LEFT
          (`SceneComponent.K2_SetWorldRotation` _paperflipbook_2 (struct :`Yaw` 90.0 :`Roll` -90.0) false false)))
      (`self.FlyTo` (`self.K2_GetActorLocation` (`self.Goal`)))
      (else
        (if (> (`KismetMathLibrary.Abs` _x) (`KismetMathLibrary.Abs` _y))
          (if (> _x 0.0)
            ;[1 0 0.8528] BACK
            (`PaperFlipbookComponent.SetFlipbook` _paperflipbook (`|GetArrayItem` _m_animations (`self.INDEX_MoveBack`)))
            (else
              ;[0 0.9771 1] FORWARD
              (`PaperFlipbookComponent.SetFlipbook` _paperflipbook (`|GetArrayItem` _m_animations (`self.INDEX_MoveFront`)))))
          (else
            (if _returnvalue
              ;[1 0.9502 0.04714] RIGHT
              (`SceneComponent.K2_SetWorldRotation` _paperflipbook (struct :`Yaw` -90.0 :`Roll` 90.0) false false)
              (else
                ;[0.01382 1 0.1518] LEFT
                (`SceneComponent.K2_SetWorldRotation` _paperflipbook (struct :`Yaw` 90.0 :`Roll` -90.0) false false)))
            (`PaperFlipbookComponent.SetFlipbook` _paperflipbook (`|GetArrayItem` _m_animations (`self.INDEX_MoveSide`)))))
        (`KismetSystemLibrary.Delay` 2.0)))))

(fn `FlyTo`
  (params (Destination :type "Vector Structure"))
  (bind (_returnvalue_x _returnvalue_y) (`KismetMathLibrary.BreakVector` (`self.K2_GetActorLocation`)))
  (bind _returnvalue (< Destination_X (- _returnvalue_x 1.0)))
  (bind _returnvalue_2 (< Destination_Y (- _returnvalue_y 1.0)))
  (`self.K2_AddActorWorldOffset` (* (* (`KismetMathLibrary.MakeVector` (select `bool` (or _returnvalue (> Destination_X (+ _returnvalue_x 1.0))) :`true` (select `bool` _returnvalue :`false` 1.0 :`true` -1.0 :!type "Float (single-precision)")) (select `bool` (or _returnvalue_2 (> Destination_Y (+ _returnvalue_y 1.0))) :`true` (select `bool` _returnvalue_2 :`false` 1.0 :`true` -1.0 :!type "Float (single-precision)"))) (`GameplayStatics.GetWorldDeltaSeconds`)) (`MovementComponent.GetMaxSpeed` (`self.FloatingPawnMovement`)))))

(fn `InitializeProperties`
  (params (RatType :type "/Game/Blueprints/Structs/STRUCT_Rat Structure") (IsUpgraded :type Boolean))
  (locals (SpawnSoundIndex :type String))
  (bind _m_animations (`self.M Animations`))
  (bind _m_animations_2 (`self.M Animations`))
  (bind _m_sounds (`self.M Sounds`))
  (bind _m_sounds_2 (`self.M Sounds`))
  (bind _m_sounds_3 (`self.M Sounds`))
  (bind _m_sounds_4 (`self.M Sounds`))
  (bind _m_sounds_5 (`self.M Sounds`))
  (bind _m_animations_3 (`self.M Animations`))
  (bind _m_sounds_6 (`self.M Sounds`))
  (bind _m_animations_4 (`self.M Animations`))
  (bind _m_sounds_7 (`self.M Sounds`))
  (bind _m_animations_5 (`self.M Animations`))
  (bind _m_sounds_8 (`self.M Sounds`))
  (bind _m_animations_6 (`self.M Animations`))
  (bind _m_sounds_9 (`self.M Sounds`))
  (bind _m_animations_7 (`self.M Animations`))
  (bind _m_animations_8 (`self.M Animations`))
  (bind _m_animations_9 (`self.M Animations`))
  (bind _value (`BlueprintMapLibrary.Map_Find` _m_sounds "NewEnumerator0"))
  (bind _value_2 (`BlueprintMapLibrary.Map_Find` _m_sounds_2 "NewEnumerator0"))
  (bind _value_3 (`BlueprintMapLibrary.Map_Find` _m_sounds_2 "NewEnumerator1"))
  (bind _value_4 (`BlueprintMapLibrary.Map_Find` _m_sounds_3 "NewEnumerator0"))
  (bind _value_5 (`BlueprintMapLibrary.Map_Find` _m_sounds_3 "NewEnumerator1"))
  (bind _value_6 (`BlueprintMapLibrary.Map_Find` _m_sounds_4 "NewEnumerator0"))
  (bind _value_7 (`BlueprintMapLibrary.Map_Find` _m_sounds_4 "NewEnumerator1"))
  (bind _value_8 (`BlueprintMapLibrary.Map_Find` _m_sounds_5 "NewEnumerator0"))
  (bind _value_9 (`BlueprintMapLibrary.Map_Find` _m_sounds_6 "NewEnumerator0"))
  (bind _value_10 (`BlueprintMapLibrary.Map_Find` _m_sounds_7 "NewEnumerator0"))
  (bind _value_11 (`BlueprintMapLibrary.Map_Find` _m_sounds_7 "NewEnumerator1"))
  (bind _value_12 (`BlueprintMapLibrary.Map_Find` _m_sounds_8 "NewEnumerator0"))
  (bind _value_13 (`BlueprintMapLibrary.Map_Find` _m_sounds_9 "NewEnumerator0"))
  (bind _value_14 (`BlueprintMapLibrary.Map_Find` _m_sounds_9 "NewEnumerator1"))
  (bind _output_get (set `self.M IsUpgraded` IsUpgraded))
  (bind _output_get_2 (set `self.M RatType` RatType))
  (`|ExecutionSequence`
    (:`then_0`
      (set `self.M Health` (`.HP_22_A5C73EA642EB0B8B3B6C66BFF461FA7C` (break `/Game/Blueprints/Structs/STRUCT_Rat` _output_get_2)))
      (set `FloatingPawnMovement.MaxSpeed` (`.Speed_24_2DE851874060508D6DA5C994695A73CC` (break `/Game/Blueprints/Structs/STRUCT_Rat` _output_get_2)) (`self.FloatingPawnMovement`))
      (set `self.M IsDying` false)
      (set `self.M IsAttacking` false)
      (bind _outactors (`GameplayStatics.GetAllActorsOfClass` "/Game/Blueprints/Actors/GameplayElement/BP_Goal.BP_Goal_C"))
      (set `self.Goal` (`|GetArrayItem` _outactors)))
    (:`then_1`
      (set `local.SpawnSoundIndex` (`|GetEnumeratorNameAsString` (break `/Game/Blueprints/Structs/STRUCT_Rat` _output_get_2)))
      (if _output_get
        (set `local.SpawnSoundIndex` (`KismetStringLibrary.Concat_StrStr` (`local.SpawnSoundIndex`) "Up")))
      (`/Game/Blueprints/Widgets/HealthBars/WBP_RatHealthBar.Initialization` :`self` (`self.HealthBarRef`) :`BarColor` (`.Color_44_0922908848A599577813F3A1BFADEA87` (break `/Game/Blueprints/Structs/STRUCT_Rat` _output_get_2))))
    (:`then_2`
      (switch `/Game/Blueprints/Enums/ENUM_RatType` (break `/Game/Blueprints/Structs/STRUCT_Rat` _output_get_2)
        (:`NewEnumerator0`
          ;[1 1 1] Grunt
          (`KismetArrayLibrary.Array_Add` _m_animations_7 "/Game/Sprites/Flipbooks/Rats/Grunt/Grunt_FrontWalk.Grunt_FrontWalk")
          (`KismetArrayLibrary.Array_Add` _m_animations_7 "/Game/Sprites/Flipbooks/Rats/Grunt/Grunt_BackWalk.Grunt_BackWalk")
          (`KismetArrayLibrary.Array_Add` _m_animations_7 "/Game/Sprites/Flipbooks/Rats/Grunt/Grunt_SideWalk.Grunt_SideWalk")
          (`KismetArrayLibrary.Array_Add` _m_animations_7 "/Game/Sprites/Flipbooks/Rats/Grunt/Grunt_Attack.Grunt_Attack")
          (`KismetArrayLibrary.Array_Add` (break `/Game/Blueprints/Structs/STRUCT_AudioContainer` _value_4) "/Game/Sounds/Rat_sounds/Grunt/Rat-Grunt-Attack-1.Rat-Grunt-Attack-1")
          (`KismetArrayLibrary.Array_Add` (break `/Game/Blueprints/Structs/STRUCT_AudioContainer` _value_4) "/Game/Sounds/Rat_sounds/Grunt/Rat-Grunt-Attack-2.Rat-Grunt-Attack-2")
          (`KismetArrayLibrary.Array_Add` (break `/Game/Blueprints/Structs/STRUCT_AudioContainer` _value_4) "/Game/Sounds/Rat_sounds/Grunt/Rat-Grunt-Attack-3.Rat-Grunt-Attack-3")
          (`KismetArrayLibrary.Array_Add` (break `/Game/Blueprints/Structs/STRUCT_AudioContainer` _value_5) "/Game/Sounds/Rat_sounds/Grunt/Rat-Grunt-kill-1.Rat-Grunt-kill-1")
          (`KismetArrayLibrary.Array_Add` (break `/Game/Blueprints/Structs/STRUCT_AudioContainer` _value_5) "/Game/Sounds/Rat_sounds/Grunt/Rat-Grunt-kill-2.Rat-Grunt-kill-2")
          (`KismetArrayLibrary.Array_Add` (break `/Game/Blueprints/Structs/STRUCT_AudioContainer` _value_5) "/Game/Sounds/Rat_sounds/Grunt/Rat-Grunt-kill-3.Rat-Grunt-kill-3")
          (`KismetArrayLibrary.Array_Add` (break `/Game/Blueprints/Structs/STRUCT_AudioContainer` _value_5) "/Game/Sounds/Rat_sounds/Grunt/Rat-Grunt-kill-4.Rat-Grunt-kill-4")
          (bind _outactors_2 (`GameplayStatics.GetAllActorsOfClass` "/Script/Engine.TargetPoint" :!label _label))
          (set `self.TargetPoint` _outactors_2))
        (:`NewEnumerator1`
          ;[1 1 1] Flying
          (if _output_get
            (`KismetArrayLibrary.Array_Add` _m_animations "/Game/Sprites/Flipbooks/Rats/FlyingUp/FlyingUp_Move.FlyingUp_Move")
            (`KismetArrayLibrary.Array_Add` _m_animations "/Game/Sprites/Flipbooks/Rats/FlyingUp/FlyingUp_Death.FlyingUp_Death")
            (`KismetArrayLibrary.Array_Add` (break `/Game/Blueprints/Structs/STRUCT_AudioContainer` _value_2) "/Game/Sounds/Rat_sounds/Flying_Rat/Rat-Flyingrat-Water-Attack-1.Rat-Flyingrat-Water-Attack-1")
            (`KismetArrayLibrary.Array_Add` (break `/Game/Blueprints/Structs/STRUCT_AudioContainer` _value_2) "/Game/Sounds/Rat_sounds/Flying_Rat/Rat-Flyingrat-Water-Attack-2.Rat-Flyingrat-Water-Attack-2")
            (`KismetArrayLibrary.Array_Add` (break `/Game/Blueprints/Structs/STRUCT_AudioContainer` _value_3) "/Game/Sounds/Rat_sounds/Flying_Rat/Rat-Flyingrat-Water-Kill-1.Rat-Flyingrat-Water-Kill-1")
            (`KismetArrayLibrary.Array_Add` (break `/Game/Blueprints/Structs/STRUCT_AudioContainer` _value_3) "/Game/Sounds/Rat_sounds/Flying_Rat/Rat-Flyingrat-Water-Kill-2.Rat-Flyingrat-Water-Kill-2")
            (else
              (`KismetArrayLibrary.Array_Add` _m_animations_6 "/Game/Sprites/Flipbooks/Rats/Flying/Flying_Move.Flying_Move")
              (`KismetArrayLibrary.Array_Add` _m_animations_6 "/Game/Sprites/Flipbooks/Rats/Flying/Flying_Death.Flying_Death")
              (`KismetArrayLibrary.Array_Add` (break `/Game/Blueprints/Structs/STRUCT_AudioContainer` _value_13) "/Game/Sounds/Rat_sounds/Flying_Rat/Rat-Flyingrat-Attack-1.Rat-Flyingrat-Attack-1")
              (`KismetArrayLibrary.Array_Add` (break `/Game/Blueprints/Structs/STRUCT_AudioContainer` _value_13) "/Game/Sounds/Rat_sounds/Flying_Rat/Rat-Flyingrat-Attack-2.Rat-Flyingrat-Attack-2")
              (`KismetArrayLibrary.Array_Add` (break `/Game/Blueprints/Structs/STRUCT_AudioContainer` _value_14) "/Game/Sounds/Rat_sounds/Flying_Rat/Rat-Flyingrat-kill-1.Rat-Flyingrat-kill-1")
              (`KismetArrayLibrary.Array_Add` (break `/Game/Blueprints/Structs/STRUCT_AudioContainer` _value_14) "/Game/Sounds/Rat_sounds/Flying_Rat/Rat-Flyingrat-kill-2.Rat-Flyingrat-kill-2")))
          (`self.K2_AddActorWorldOffset` (0.0 0.0 350.0))
          (`PaperFlipbookComponent.SetFlipbook` (`self.PaperFlipbook`) (`|GetArrayItem` (`self.M Animations`))))
        (:`NewEnumerator6`
          ;[1 1 1] Tank
          (if _output_get
            (`KismetArrayLibrary.Array_Add` _m_animations_8 "/Game/Sprites/Rats/TankUp/TankUp_FrontWalk.TankUp_FrontWalk")
            (`KismetArrayLibrary.Array_Add` _m_animations_8 "/Game/Sprites/Flipbooks/Rats/Tank/Tank_BackWalk.Tank_BackWalk")
            (`KismetArrayLibrary.Array_Add` _m_animations_8 "/Game/Sprites/Rats/TankUp/TankUp_SideWalk.TankUp_SideWalk")
            (`KismetArrayLibrary.Array_Add` _m_animations_8 "/Game/Sprites/Rats/TankUp/TankUp_Attack.TankUp_Attack")
            (`KismetArrayLibrary.Array_Add` _m_animations_8 "/Game/Sprites/Rats/TankUp/TankUp_Death.TankUp_Death")
            (`KismetArrayLibrary.Array_Add` (break `/Game/Blueprints/Structs/STRUCT_AudioContainer` _value) "/Game/Sounds/Rat_Sound_-_Tank/Tank/Rat-Tank-Earth-Attack-1.Rat-Tank-Earth-Attack-1")
            (`KismetArrayLibrary.Array_Add` (break `/Game/Blueprints/Structs/STRUCT_AudioContainer` _value) "/Game/Sounds/Rat_Sound_-_Tank/Tank/Rat-Tank-Earth-Attack-2.Rat-Tank-Earth-Attack-2")
            (`KismetArrayLibrary.Array_Add` (break `/Game/Blueprints/Structs/STRUCT_AudioContainer` (`BlueprintMapLibrary.Map_Find` _m_sounds "NewEnumerator1")) "/Game/Sounds/Rat_Sound_-_Tank/Tank/Rat-Tank-Earth-Kill.Rat-Tank-Earth-Kill")
            (goto _label)
            (else
              (`KismetArrayLibrary.Array_Add` _m_animations_3 "/Game/Sprites/Flipbooks/Rats/Tank/Tank_FrontWalk.Tank_FrontWalk")
              (`KismetArrayLibrary.Array_Add` _m_animations_3 "/Game/Sprites/Flipbooks/Rats/Tank/Tank_BackWalk.Tank_BackWalk")
              (`KismetArrayLibrary.Array_Add` _m_animations_3 "/Game/Sprites/Flipbooks/Rats/Tank/Tank_SideWalk.Tank_SideWalk")
              (`KismetArrayLibrary.Array_Add` _m_animations_3 "/Game/Sprites/Flipbooks/Rats/Tank/Tank_Attack.Tank_Attack")
              (`KismetArrayLibrary.Array_Add` _m_animations_3 "/Game/Sprites/Flipbooks/Rats/Tank/Tank_Death.Tank_Death")
              (`KismetArrayLibrary.Array_Add` (break `/Game/Blueprints/Structs/STRUCT_AudioContainer` _value_9) "/Game/Sounds/Rat_Sound_-_Tank/Tank/Rat-Tank-Attack-1.Rat-Tank-Attack-1")
              (`KismetArrayLibrary.Array_Add` (break `/Game/Blueprints/Structs/STRUCT_AudioContainer` _value_9) "/Game/Sounds/Rat_Sound_-_Tank/Tank/Rat-Tank-Attack-2.Rat-Tank-Attack-2")
              (`KismetArrayLibrary.Array_Add` (break `/Game/Blueprints/Structs/STRUCT_AudioContainer` (`BlueprintMapLibrary.Map_Find` _m_sounds_6 "NewEnumerator1")) "/Game/Sounds/Rat_Sound_-_Tank/Tank/Rat-Tank-Kill.Rat-Tank-Kill")
              (goto _label))))
        (:`NewEnumerator2`
          ;[1 1 1] Speed
          (if _output_get
            (`KismetArrayLibrary.Array_Add` _m_animations_9 "/Game/Sprites/Flipbooks/Rats/SpeedUp/SpeedUp_FrontWalk.SpeedUp_FrontWalk")
            (`KismetArrayLibrary.Array_Add` _m_animations_9 "/Game/Sprites/Flipbooks/Rats/SpeedUp/SpeedUp_BackWalk.SpeedUp_BackWalk")
            (`KismetArrayLibrary.Array_Add` _m_animations_9 "/Game/Sprites/Flipbooks/Rats/SpeedUp/SpeedUp_SideWalk.SpeedUp_SideWalk")
            (`KismetArrayLibrary.Array_Add` _m_animations_9 "/Game/Sprites/Flipbooks/Rats/SpeedUp/SpeedUp_Attack.SpeedUp_Attack")
            (`KismetArrayLibrary.Array_Add` _m_animations_9 "/Game/Sprites/Flipbooks/Rats/SpeedUp/SpeedUp_Death.SpeedUp_Death")
            (`KismetArrayLibrary.Array_Add` (break `/Game/Blueprints/Structs/STRUCT_AudioContainer` _value_6) "/Game/Sounds/Rat_sounds/Speed_Rat/Rat-Speedrat-Fire-Attack-1.Rat-Speedrat-Fire-Attack-1")
            (`KismetArrayLibrary.Array_Add` (break `/Game/Blueprints/Structs/STRUCT_AudioContainer` _value_6) "/Game/Sounds/Rat_sounds/Speed_Rat/Rat-Speedrat-Fire-Attack-2.Rat-Speedrat-Fire-Attack-2")
            (`KismetArrayLibrary.Array_Add` (break `/Game/Blueprints/Structs/STRUCT_AudioContainer` _value_7) "/Game/Sounds/Rat_sounds/Speed_Rat/Rat-Speedrat-Fire-Kill-1.Rat-Speedrat-Fire-Kill-1")
            (`KismetArrayLibrary.Array_Add` (break `/Game/Blueprints/Structs/STRUCT_AudioContainer` _value_7) "/Game/Sounds/Rat_sounds/Speed_Rat/Rat-Speedrat-Fire-Kill-2.Rat-Speedrat-Fire-Kill-2")
            (goto _label)
            (else
              (`KismetArrayLibrary.Array_Add` _m_animations_4 "/Game/Sprites/Flipbooks/Rats/Speed/Speed_FrontWalk.Speed_FrontWalk")
              (`KismetArrayLibrary.Array_Add` _m_animations_4 "/Game/Sprites/Flipbooks/Rats/Speed/Speed_BackWalk.Speed_BackWalk")
              (`KismetArrayLibrary.Array_Add` _m_animations_4 "/Game/Sprites/Flipbooks/Rats/Speed/Speed_SideWalk.Speed_SideWalk")
              (`KismetArrayLibrary.Array_Add` _m_animations_4 "/Game/Sprites/Flipbooks/Rats/Speed/Speed_Attack.Speed_Attack")
              (`KismetArrayLibrary.Array_Add` _m_animations_4 "/Game/Sprites/Flipbooks/Rats/Speed/Speed_Death.Speed_Death")
              (`KismetArrayLibrary.Array_Add` (break `/Game/Blueprints/Structs/STRUCT_AudioContainer` _value_10) "/Game/Sounds/Rat_sounds/Speed_Rat/Rat-Speedrat-Attack-1.Rat-Speedrat-Attack-1")
              (`KismetArrayLibrary.Array_Add` (break `/Game/Blueprints/Structs/STRUCT_AudioContainer` _value_10) "/Game/Sounds/Rat_sounds/Speed_Rat/Rat-Speedrat-Attack-2.Rat-Speedrat-Attack-2")
              (`KismetArrayLibrary.Array_Add` (break `/Game/Blueprints/Structs/STRUCT_AudioContainer` _value_11) "/Game/Sounds/Rat_sounds/Speed_Rat/Rat-Speedrat-Kill-1.Rat-Speedrat-Kill-1")
              (`KismetArrayLibrary.Array_Add` (break `/Game/Blueprints/Structs/STRUCT_AudioContainer` _value_11) "/Game/Sounds/Rat_sounds/Speed_Rat/Rat-Speedrat-Kill-2.Rat-Speedrat-Kill-2")
              (goto _label))))
        (:`NewEnumerator3`
          ;[1 1 1] Ninja
          (if _output_get
            (`KismetArrayLibrary.Array_Add` _m_animations_2 "/Game/Sprites/Flipbooks/Rats/Ninja/Ninja_FrontWalk.Ninja_FrontWalk")
            (`KismetArrayLibrary.Array_Add` _m_animations_2 "/Game/Sprites/Flipbooks/Rats/Ninja/Ninja_BackWalk.Ninja_BackWalk")
            (`KismetArrayLibrary.Array_Add` _m_animations_2 "/Game/Sprites/Flipbooks/Rats/Ninja/Ninja_SideWalk.Ninja_SideWalk")
            (`KismetArrayLibrary.Array_Add` _m_animations_2 "/Game/Textures/Rats/NinjaUp/NinjaUp_Attack.NinjaUp_Attack")
            (`KismetArrayLibrary.Array_Add` _m_animations_2 "/Game/Sprites/Flipbooks/Rats/Ninja/Ninja_Death.Ninja_Death")
            (`KismetArrayLibrary.Array_Add` (break `/Game/Blueprints/Structs/STRUCT_AudioContainer` _value_8) "/Game/Sounds/Ninja/Ninja/Rat-Ninja-Wind-Attack-1.Rat-Ninja-Wind-Attack-1")
            (`KismetArrayLibrary.Array_Add` (break `/Game/Blueprints/Structs/STRUCT_AudioContainer` _value_8) "/Game/Sounds/Ninja/Ninja/Rat-Ninja-Wind-Attack-2.Rat-Ninja-Wind-Attack-2")
            (`KismetArrayLibrary.Array_Add` (break `/Game/Blueprints/Structs/STRUCT_AudioContainer` (`BlueprintMapLibrary.Map_Find` _m_sounds_5 "NewEnumerator1")) "/Game/Sounds/Ninja/Ninja/Rat-Ninja-Wind-Kill.Rat-Ninja-Wind-Kill")
            (goto _label)
            (else
              (`KismetArrayLibrary.Array_Add` _m_animations_5 "/Game/Sprites/Flipbooks/Rats/Ninja/Ninja_FrontWalk.Ninja_FrontWalk")
              (`KismetArrayLibrary.Array_Add` _m_animations_5 "/Game/Sprites/Flipbooks/Rats/Ninja/Ninja_BackWalk.Ninja_BackWalk")
              (`KismetArrayLibrary.Array_Add` _m_animations_5 "/Game/Sprites/Flipbooks/Rats/Ninja/Ninja_SideWalk.Ninja_SideWalk")
              (`KismetArrayLibrary.Array_Add` _m_animations_5 "/Game/Sprites/Flipbooks/Rats/Ninja/Ninja_Attack.Ninja_Attack")
              (`KismetArrayLibrary.Array_Add` _m_animations_5 "/Game/Sprites/Flipbooks/Rats/Ninja/Ninja_Death.Ninja_Death")
              (`KismetArrayLibrary.Array_Add` (break `/Game/Blueprints/Structs/STRUCT_AudioContainer` _value_12) "/Game/Sounds/Ninja/Ninja/Rat-Ninja-Attack-1.Rat-Ninja-Attack-1")
              (`KismetArrayLibrary.Array_Add` (break `/Game/Blueprints/Structs/STRUCT_AudioContainer` _value_12) "/Game/Sounds/Ninja/Ninja/Rat-Ninja-Attack-2.Rat-Ninja-Attack-2")
              (`KismetArrayLibrary.Array_Add` (break `/Game/Blueprints/Structs/STRUCT_AudioContainer` (`BlueprintMapLibrary.Map_Find` _m_sounds_8 "NewEnumerator1")) "/Game/Sounds/Ninja/Ninja/Rat-Ninja-Kill.Rat-Ninja-Kill")
              (goto _label)))))
      (`AudioComponent.SetSound` (`self.Channel_Event`) (`self.RandomSoundFrom` (break `/Game/Blueprints/Structs/STRUCT_AudioContainer` (`BlueprintMapLibrary.Map_Find` (`self.GetSpawnSoundsSTDs`) (`local.SpawnSoundIndex`)))))
      (`AudioComponent.Play` (`self.Channel_Event`) 0.0)
      (set `self.GoalPos` (`self.K2_GetActorLocation` (`self.Goal`)))
      (`self.Movement`))))

(fn `ReceiveDamages`
  (params (DamagesAmount :type "Float (double-precision)") (SlowForce :type "Float (double-precision)") (SlowDuration :type "Float (double-precision)"))
  (returns (StillAlive :type Boolean))
  (bind _return (`self.HealthBarRef`))
  (bind _m_animations (`self.M Animations`))
  (bind _m_rattype_type (break `/Game/Blueprints/Structs/STRUCT_Rat` (`self.M RatType`)))
  (bind _channel_event_bis (`self.Channel_Event_bis`))
  (bind _floatingpawnmovement (`self.FloatingPawnMovement`))
  (bind _returnvalue (- (`self.M Health`) DamagesAmount))
  (bind _returnvalue_2 (<= _returnvalue 0.0))
  (if (<= SlowForce 1.0)
    (if (not (`self.M IsSlowed`))
      (set `FloatingPawnMovement.MaxSpeed` (* (`FloatingPawnMovement.MaxSpeed` _floatingpawnmovement) (- 1.0 SlowForce)) _floatingpawnmovement)
      (set `self.M SlowDuration` SlowDuration)
      (set `self.M IsSlowed` true)))
  (if (not _returnvalue_2)
    (`/Game/Blueprints/Widgets/HealthBars/WBP_RatHealthBar.RefreshHpLoss` _return (`KismetMathLibrary.FTrunc` DamagesAmount)))
  (bind _output_get (set `self.M Health` _returnvalue))
  (set `/Game/Blueprints/Widgets/HealthBars/WBP_RatHealthBar.M Health` _output_get _return)
  (if _returnvalue_2
    (set `self.M IsDying` true)
    (`AudioComponent.SetSound` _channel_event_bis (`self.RandomSoundFrom` (break `/Game/Blueprints/Structs/STRUCT_AudioContainer` (`BlueprintMapLibrary.Map_Find` (`self.M Sounds`) "NewEnumerator1"))))
    (`AudioComponent.Play` _channel_event_bis 0.0)
    (`PaperFlipbookComponent.SetFlipbook` (`self.PaperFlipbook`) (select `bool` (`|EnumEquality` _m_rattype_type "NewEnumerator1") :`false` (`|GetArrayItem` _m_animations (`self.INDEX_Death`)) :`true` (`|GetArrayItem` _m_animations 1)))
    (return false)
    (else
      (return true))))

(fn `UserConstructionScript`
  (bind _paperflipbook (`self.PaperFlipbook`))
  (`SceneComponent.K2_SetWorldRotation` _paperflipbook (struct :`Yaw` -90.0 :`Roll` 90.0) false false)
  (`SceneComponent.SetWorldScale3D` _paperflipbook (0.2 0.2 0.2)))